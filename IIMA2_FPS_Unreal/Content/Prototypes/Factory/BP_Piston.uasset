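; Factory prototype piston that pushes its head downward and then retracts it, once after play begins.
; BeginPlay starts a timer that plays the push timeline and schedules a second timer for the retract timeline, which does not re-arm the push.
; Both timelines drive the head's relative Z with swept moves.
; Two getters report the piston as mobile with a downward move direction.
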(event Custom|proxy_PushTimer
  (bind _pistonhead (Variables|Default|GetPistonHead))
  (bind _relativelocation (Variables|/Script/Engine.SceneComponent|GetRelativeLocation _pistonhead))
  (Utilities|Time|ClearandInvalidateTimerbyHandle (Variables|Default|GetPushTimer))
  (bind _returnvalue (Utilities|Time|SetTimerbyEvent (delegate Custom|proxy_RetractTimer) 2.5))
  (Variables|Default|SetRetractTimer _returnvalue)
  (bind _newtrack_0 (Timeline|PushTimeLine Play)
    (:Update
      (Transformation|SetRelativeLocation _pistonhead (Math|Vector|MakeVector (.x _relativelocation) (.y _relativelocation) (+ 0.0 (Math|Float|Lerp 0.0 -1e+02 _newtrack_0))) true false))))

(event Custom|proxy_RetractTimer
  (bind _pistonhead (Variables|Default|GetPistonHead))
  (bind _relativelocation (Variables|/Script/Engine.SceneComponent|GetRelativeLocation _pistonhead))
  (Utilities|Time|ClearandInvalidateTimerbyHandle (Variables|Default|GetRetractTimer))
  (bind _newtrack_0 (Timeline|RetractTimeline Play)
    (:Update
      (Transformation|SetRelativeLocation _pistonhead (Math|Vector|MakeVector (.x _relativelocation) (.y _relativelocation) _newtrack_0) true false))))

(event EventBeginPlay
  (bind _returnvalue (Utilities|Time|SetTimerbyEvent (delegate Custom|proxy_PushTimer) 2.0))
  (Variables|Default|SetPushTimer _returnvalue))

(fn ConstructionScript)

(fn GetIsMobile
  (return true))

(fn GetMoveDirection
  (return "0.000000,0.000000,-1.000000"))