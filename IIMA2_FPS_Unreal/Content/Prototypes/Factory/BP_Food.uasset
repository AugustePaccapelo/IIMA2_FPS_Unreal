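; BP_Food is a factory prototype food item that gets crushed into BP_FoodBis by moving building structures.
; When a mobile BPI_BuildingStructure actor hits its Box, a line trace along the hit normal checks for a blocking object.
; If blocked, the Box's Z scale shrinks using the DeltaSeconds cached on Tick.
; Once squashed below a threshold, it spawns BP_FoodBis in its place and destroys itself.
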(event OnComponentHit(Cube)
  (params (HitComponent :type Primitive%20Component%20Object%20Reference) (OtherActor :type Actor%20Object%20Reference) (OtherComp :type Primitive%20Component%20Object%20Reference) (NormalImpulse :type Vector :default "0, 0, 0") (Hit :type Hit%20Result%20Structure%20%28by%20ref%29)))

(event OnComponentHit(Box)
  (params (HitComponent :type Primitive%20Component%20Object%20Reference) (OtherActor :type Actor%20Object%20Reference) (OtherComp :type Primitive%20Component%20Object%20Reference) (NormalImpulse :type Vector :default "0, 0, 0") (Hit :type Hit%20Result%20Structure%20%28by%20ref%29))
  (bind _returnvalue (Transformation|GetActorLocation))
  (bind _returnvalue_2 (Transformation|GetActorTransform))
  (bind _delta_seconds (Variables|Default|GetDelta%20Seconds))
  (bind _box (Variables|Default|GetBox))
  (bind _returnvalue_3 (* _delta_seconds 1.0))
  (bind _relativescale3d (Variables|/Script/Engine.SceneComponent|GetRelativeScale3D _box))
  (bind _returnvalue_4 (- (.z _relativescale3d) _returnvalue_3))
  (bind _returnvalue_5 (Math|Float|Clamp(Float) _returnvalue_4 0.1 1.5))
  (if (Utilities|DoesObjectImplementInterface OtherActor "/Game/Prototypes/Factory/BPI_BuildingStructure.BPI_BuildingStructure_C")
    (bind _ismobile (Class|BPIBuildingStructure|GetIsMobile(Message) OtherActor))
    (if _ismobile
      (bind _returnvalue_6 (Collision|LineTraceByChannel _returnvalue (+ _returnvalue (* (.normal Hit) (Variables|Default|GetTraceDist))) "TraceTypeQuery3" false 0 "None"))
      (if _returnvalue_6
        (Transformation|SetRelativeScale3D _box (Math|Vector|MakeVector (.x _relativescale3d) (.y _relativescale3d) _returnvalue_5))
        (if (< _returnvalue_5 0.5)
          (Game|SpawnActorfromClass "/Game/Prototypes/Factory/BP_FoodBis.BP_FoodBis_C" (Math|Transform|MakeTransform (.location _returnvalue_2) (.rotation _returnvalue_2) "1.000000,1.000000,1.000000") "Undefined" "MultiplyWithRoot" 0 0)
          (Actor|DestroyActor))))))

(event EventBeginPlay)

(event Collision|EventActorBeginOverlap
  (params (OtherActor :type Actor%20Object%20Reference)))

(event EventTick
  (params (DeltaSeconds :type Float%20%28single-precision%29))
  (Variables|Default|SetDelta%20Seconds DeltaSeconds))

(fn ConstructionScript)