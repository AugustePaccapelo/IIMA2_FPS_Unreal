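; BP_MovableLasersWay is a trap actor that spawns a row of laser actors along a spline.
; On BeginPlay it loops over LasersNumber, spacing spawn points by spline length divided by that count.
; A switch on LaserType picks the laser, with only the Ejection case spawning anything (BP_LaserEjection).
; Spawn transforms are read in the spline's local space, and nothing here moves the lasers afterward.
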(event EventBeginPlay
  (for _index (range 0 (Variables|Default|GetlasersNumber))
    (switch Utilities|FlowControl|Switch|SwitchonE_LaserType (Variables|Default|GetLaserType)
      (:NewEnumerator0
        (Game|SpawnActorfromClass "/Game/BluePrints/Traps/Lasers/BP_LaserEjection.BP_LaserEjection_C" (Spline|GetTransformatDistanceAlongSpline (Variables|Default|GetSpline) (Math|Conversions|ToFloat(Integer) (* _index (/ (Spline|GetSplineLength (Variables|Default|GetSpline)) (Variables|Default|GetlasersNumber)))) "Local" false) "Undefined" "MultiplyWithRoot" 0 0)))))

(fn ConstructionScript)