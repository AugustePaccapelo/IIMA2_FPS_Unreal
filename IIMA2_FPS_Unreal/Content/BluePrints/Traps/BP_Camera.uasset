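; BP_Camera is a security camera trap whose spotlight marks its detection zone.
; The construction script rotates, scales and positions a Cone mesh to match the spotlight's beam, deriving its size from outer cone angle and attenuation radius.
; Overlapping the cone fires a visibility line trace from the spotlight, intended to check for walls before triggering defeat.
; The trace has no end point wired, and its result triggers nothing yet.
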(event OnComponentBeginOverlap(Cone)
  (params (OverlappedComponent :type Primitive%20Component%20Object%20Reference) (OtherActor :type Actor%20Object%20Reference) (OtherComp :type Primitive%20Component%20Object%20Reference) (OtherBodyIndex :type Integer) (bFromSweep :type Boolean) (SweepResult :type Hit%20Result%20Structure%20%28by%20ref%29))
  ;[0.15 0.04 0.03506 0.5] Si le joueur est detecté dans l'overlap on retrace un trait entre lui et le cone pour verifier qu'il y a pas un mur ou autre entre les deux puis on déclenche la défaite
  (bind _returnvalue (Collision|LineTraceByChannel (Transformation|GetWorldLocation (Variables|Default|GetSpotLight)) "0, 0, 0" "TraceTypeQuery1" false 0 "None"))
  (if _returnvalue
    _))

(fn ConstructionScript
  (bind _spotlight (Variables|Default|GetSpotLight))
  (bind _spotlight_2 (Variables|Default|GetSpotLight))
  (bind _returnvalue (Transformation|GetWorldRotation _spotlight))
  (bind _attenuationradius (Variables|/Script/Engine.LocalLightComponent|GetAttenuationRadius _spotlight))
  (bind _outerconeangle (Variables|/Script/Engine.SpotLightComponent|GetOuterConeAngle _spotlight))
  (bind _returnvalue_2 (Math|Trig|Tan(Degrees) _outerconeangle))
  (bind _returnvalue_3 (/ _attenuationradius 1e+02))
  (bind _returnvalue_4 (* _returnvalue_2 _returnvalue_3))
  (bind _returnvalue_5 (* _returnvalue_4 2.0))
  (Transformation|SetWorldRotation (Variables|Default|GetCone) (Math|Rotator|MakeRotator (.roll _returnvalue) (+ (.pitch _returnvalue) 9e+01) (.yaw _returnvalue)) false false)
  (Transformation|SetWorldScale3D (Variables|Default|GetCone) (Math|Vector|MakeVector _returnvalue_5 _returnvalue_5 _returnvalue_3))
  (Transformation|SetWorldLocation (Variables|Default|GetCone) (+ (Transformation|GetWorldLocation _spotlight_2) (* (Math|Vector|GetForwardVector _spotlight_2) (/ _attenuationradius 2.0))) false false))