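; Laser trap Blueprint whose beam stretches between blocking surfaces, up to a maximum length.
; The Construction Script computes both maximum endpoints along the laser's up axis and line-traces on Visibility to fix the upper one.
; Each Tick re-traces from just off that point toward the lower limit, then rescales the beam's Z and centers it between the hits.
; The overlap event intended for player detection is empty.
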(event OnComponentBeginOverlap(Laser)
  (params (OverlappedComponent :type Primitive%20Component%20Object%20Reference) (OtherActor :type Actor%20Object%20Reference) (OtherComp :type Primitive%20Component%20Object%20Reference) (OtherBodyIndex :type Integer) (bFromSweep :type Boolean) (SweepResult :type Hit%20Result%20Structure%20%28by%20ref%29))
  ;[0.15 0.03604 0.04742 0.5] Detection du joueur
)

(event EventTick
  (params (DeltaSeconds :type Float%20%28single-precision%29))
  ;[0.15 0.15 0.15 0.5 15] Update de la longueur du laser (si ya des elements qui bloquent le laser)
  (CallFunction|SetLaserScale))

(fn ConstructionScript
  (bind _laser (Variables|Default|GetLaser))
  (bind _lasermaxlenght (Variables|Default|GetlaserMaxLenght))
  (bind _returnvalue (Math|Vector|GetUpVector _laser))
  (bind _returnvalue_2 (/ _lasermaxlenght 2.0))
  (bind _returnvalue_3 (* _returnvalue _returnvalue_2))
  ;[0.15 0.08528 0.1262 0.5] Point max a atteindre vers le haut et vers le bas
  (Variables|Default|SetlaseMaxUpPoint (+ _returnvalue_3 (Transformation|GetWorldLocation (Variables|Default|GetLaser))))
  (Variables|Default|SetlaseMaxDownPoint (+ (* _returnvalue_3 -1.0) (Transformation|GetWorldLocation (Variables|Default|GetLaser))))
  (bind _point (CallFunction|GetLaserHitPoint (Transformation|GetWorldLocation (Variables|Default|GetLaser)) (Variables|Default|GetlaseMaxUpPoint)))
  ;[0.15 0.1168 0.04254 0.5] Calcul de la taille du laser
  (Variables|Default|SetupPoint _point)
  (CallFunction|SetLaserScale))

(fn GetLaserHitPoint
  (params (startPoint :type Vector) (maxEndPoint :type Vector))
  (bind (_outhit _returnvalue) (Collision|LineTraceByChannel startPoint maxEndPoint "TraceTypeQuery1" false 0 "None"))
  (if _returnvalue
    (return (.ImpactPoint (Collision|BreakHitResult _outhit)))
    (else
      (return maxEndPoint))))

(fn SetLaserScale
  (bind _uppoint (Variables|Default|GetupPoint))
  (bind _laser (Variables|Default|GetLaser))
  (bind _returnvalue (Transformation|GetWorldScale _laser))
  (bind _point (CallFunction|GetLaserHitPoint (Math|Vector|MakeVector (- (.x _uppoint) 0.2) (- (.y _uppoint) 0.2) (- (.z _uppoint) 0.2)) (Variables|Default|GetlaseMaxDownPoint)))
  (Variables|Default|SetdownPoint _point)
  (Transformation|SetWorldScale3D _laser (Math|Vector|MakeVector (.x _returnvalue) (.y _returnvalue) (/ (Math|Vector|Distance(Vector) (Variables|Default|GetupPoint) (Variables|Default|GetdownPoint)) 1e+02)))
  ;[0.05981 0.15 0.07225 0.5] Calcul de la position du laser
  (Transformation|SetWorldLocation (Variables|Default|GetLaser) (/ (+ (Variables|Default|GetupPoint) (Variables|Default|GetdownPoint)) 2.0) false false))