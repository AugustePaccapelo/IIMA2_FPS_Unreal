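; HUD_Game is the game HUD that puts the main interface on screen and handles toggling of the pause menu.
; BeginPlay constructs WBP_Main and adds it to the viewport.
; The OpenMenu event alternates through a FlipFlop between creating WBP_PauseMenu with UI-only input and removing it with game-only input.
; The pause widget is not added to the viewport in this graph, and game pause is not set here.
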(event Custom|OpenMenu
  (bind _returnvalue (Game|GetPlayerController 0))
  (Utilities|FlowControl|FlipFlop
    (:A
      ;[0.1067 0.15 0.06352 0.5] ouverture du menu
      (Input|SetInputModeUIOnly _returnvalue 0 "DoNotLock" false)
      (bind _returnvalue_2 (UserInterface|CreateWidget "/Game/Widgets/WBP_PauseMenu.WBP_PauseMenu_C"))
      (Variables|Default|SetPauseMenuWidget _returnvalue_2))
    (:B
      ;[0.15 0.04391 0.04391 0.5] fermeture du menu
      (Input|SetInputModeGameOnly _returnvalue false)
      (Widget|RemovefromParent (Variables|Default|GetPauseMenuWidget)))))

(event EventBeginPlay
  ;[0.03326 0.07269 0.15 0.5] affichage de l'HUD
  (bind _returnvalue (Game|ConstructObjectfromClass "/Game/Widgets/WBP_Main.WBP_Main_C"))
  (bind _output_get (Variables|Default|SetmainCanvas _returnvalue))
  (UserInterface|Viewport|AddtoViewport _output_get 0))

(fn ConstructionScript)