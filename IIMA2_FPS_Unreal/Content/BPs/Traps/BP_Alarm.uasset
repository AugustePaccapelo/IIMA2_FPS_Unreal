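; Alarm trap that, when triggered, reports a noise event at its sound location and starts a pulsing light with a Niagara effect.
; Fade-in and fade-out timelines drive a weight that lerps point light intensity, repeating after a delay while the alarm is on.
; BeginPlay injects the fade curves and scales playback by sequence duration.
; TurnOff clears the on flag and stops both timelines, leaving Niagara untouched.
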(event Custom|CE_StartIn
  (Components|Activation|Activate (Variables|Default|GetNiagara) false)
  ;[0.15 0.15 0.15 0.5] TimeLines
  ;;[0.15 0.15 0.15 0.5] FadeIn
  (bind _fadetrack (Timeline|TL_Light_In PlayFromStart)
    (:Update
      (Variables|Light|SetWeigth _fadetrack)
      (CallFunction|UpdateIntensity))
    (:Finished
      (CallFunction|CEStartOut))))

(event Custom|CE_StartOut
  ;[0.15 0.15 0.15 0.5] TimeLines
  ;;[0.15 0.15 0.15 0.5] FadeOut
  (bind _fadetrack (Timeline|TL_Light_Out PlayFromStart)
    (:Update
      (Variables|Light|SetWeigth _fadetrack)
      (CallFunction|UpdateIntensity))
    (:Finished
      (if (Variables|Light|GetIsOn)
        (Utilities|FlowControl|Delay (Variables|Light|GetTimeBetweenCicles))
        (CallFunction|Turnon)))))

(event EventBeginPlay
  ;[0.15 0.15 0.15 0.5] BeginPlay, set up variables
  (|CallParentFunction)
  (Class|TimelineComponent|SetFloatCurve (Variables|Default|GetTL_Light_In) (Variables|Light|GetFadeIn) (Variables|Light|GetTrackNames))
  (Class|TimelineComponent|SetFloatCurve (Variables|Default|GetTL_Light_Out) (Variables|Light|GetFadeOut) (Variables|Light|GetTrackNames))
  (Components|Timeline|SetPlayRate (Variables|Default|GetTL_Light_In) (/ 2.0 (Variables|Light|GetSequenceDuration)))
  (Components|Timeline|SetPlayRate (Variables|Default|GetTL_Light_Out) (/ 2.0 (Variables|Light|GetSequenceDuration)))
  (Variables|Light|SetWeigth 0.0)
  (CallFunction|UpdateIntensity)
  (Components|Activation|Deactivate (Variables|Default|GetNiagara)))

(event EventTrigger
  ;[0.15 0.15 0.15 0.5] TrapTrigger
  (Class|AISenseHearing|ReportNoiseEvent (Transformation|GetWorldLocation (Variables|Default|GetSoundLocation)) (Variables|Trap|GetLoudness) self (* (Variables|Trap|GetMaxRange) 1e+02) (Variables|Trap|GetTag))
  (CallFunction|Turnon))

(fn ConstructionScript
  (|CallParentFunction))

(fn Turnon
  (Variables|Light|SetIsOn true)
  (CallFunction|CEStartin))

(fn TurnOff
  (Variables|Light|SetIsOn false)
  (Audio|Components|Audio|Stop (Variables|Default|GetTL_Light_In))
  (Audio|Components|Audio|Stop (Variables|Default|GetTL_Light_Out)))

(fn UpdateIntensity
  (Rendering|Components|Light|SetIntensity (Variables|Default|GetPointLight) (Math|Float|Lerp (Variables|Light|GetMinLightIntensity) (Variables|Light|GetMaxLightIntensity) (Variables|Light|GetWeigth))))