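; BP_BlackHole is a trap that drags BP_Player toward its center and ends the game as a loss when the player gets too close.
; Overlapping the BlackHoleRange sphere enables a per-tick pull that damps velocity and adds attraction inversely proportional to distance.
; Max speed also lerps toward zero nearer the center, and is restored on leaving the sphere.
; Within DeathDistance, it calls FinishGame on GI_Main and stops the player.
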(event OnComponentBeginOverlap(BlackHoleRange)
  (params (OverlappedComponent :type Primitive%20Component%20Object%20Reference) (OtherActor :type Actor%20Object%20Reference) (OtherComp :type Primitive%20Component%20Object%20Reference) (OtherBodyIndex :type Integer) (bFromSweep :type Boolean) (SweepResult :type Hit%20Result%20Structure%20%28by%20ref%29))
  (bind _asbp_player (Utilities|Casting|CastToBP_Player OtherActor))
  (Variables|Refs|SetAs%20BP%20Player _asbp_player)
  (Variables|Default|SetCanAttractPlayer true)
  (Development|PrintString "joueur dans trou noir"))

(event OnComponentEndOverlap(BlackHoleRange)
  (params (OverlappedComponent :type Primitive%20Component%20Object%20Reference) (OtherActor :type Actor%20Object%20Reference) (OtherComp :type Primitive%20Component%20Object%20Reference) (OtherBodyIndex :type Integer))
  (bind _asbp_player (Utilities|Casting|CastToBP_Player OtherActor))
  (Variables|Default|SetCanAttractPlayer false)
  (Variables|/Script/Engine.FloatingPawnMovement|SetMaxSpeed (Variables|/Game/BPs/BP_Player.BP_Player_C|GetFloatingPawnMovement _asbp_player) (Variables|Default|GetPlayerMaxSpeed)))

(event Custom|StopPlayer
  (bind _as_bp_player (Variables|Refs|GetAs%20BP%20Player))
  ;[0.15 0.15 0.15 0.5] stopper le joueur a la mort
  (Utilities|IsValid _as_bp_player
    (:Is%20Valid
      (Components|Movement|StopMovementImmediately (Variables|/Game/BPs/BP_Player.BP_Player_C|GetFloatingPawnMovement _as_bp_player)))))

(event EventBeginPlay
  (bind _asgi_main (Utilities|Casting|CastToGI_Main (Game|GetGameInstance)))
  (Variables|Refs|SetAs%20GI%20Main _asgi_main)
  (bind _asbp_player (Utilities|Casting|CastToBP_Player (Game|Player|GetPlayerPawn 0)))
  (Variables|Default|SetPlayerMaxSpeed (Class|MovementComponent|GetMaxSpeed (Variables|/Game/BPs/BP_Player.BP_Player_C|GetFloatingPawnMovement _asbp_player))))

(event EventTick
  (params (DeltaSeconds :type Float%20%28single-precision%29))
  (bind _as_bp_player (Variables|Refs|GetAs%20BP%20Player))
  (bind _floatingpawnmovement (Variables|/Game/BPs/BP_Player.BP_Player_C|GetFloatingPawnMovement _as_bp_player))
  (if (Variables|Default|GetCanAttractPlayer)
    (Utilities|IsValid _as_bp_player
      (:Is%20Valid
        (Variables|Default|SetPlayerDistance (Math|Vector|Distance(Vector) (Transformation|GetWorldLocation (Variables|Default|GetBlackHole)) (Transformation|GetActorLocation (Variables|Refs|GetAs%20BP%20Player))))
        (Variables|/Script/Engine.MovementComponent|SetVelocity _floatingpawnmovement (+ (* (Variables|/Script/Engine.MovementComponent|GetVelocity _floatingpawnmovement) 0.98) (* (Math|Vector|Normalize (- (Transformation|GetWorldLocation (Variables|Default|GetBlackHole)) (Transformation|GetActorLocation (Variables|Refs|GetAs%20BP%20Player)))) DeltaSeconds (/ (Variables|Settings|GetAttractionForce) (Variables|Default|GetPlayerDistance)))))
        ;[0.15 0.0739 0.1443 0.5] On reduit la vitesse de notre joueur pour qu'il ait de plus en plus de mal a se degager
        (Variables|Default|SetSpeedAlpha (- 1.0 (/ (Variables|Default|GetPlayerDistance) (Variables|/Script/Engine.SphereComponent|GetSphereRadius (Variables|Default|GetBlackHoleRange)))))
        (Utilities|String|LogString (Utilities|String|ToString(Float) (Math|Float|Lerp (Variables|Default|GetPlayerMaxSpeed) 0.0 (Variables|Default|GetSpeedAlpha))))
        (Variables|/Script/Engine.FloatingPawnMovement|SetMaxSpeed (Variables|/Game/BPs/BP_Player.BP_Player_C|GetFloatingPawnMovement (Variables|Refs|GetAs%20BP%20Player)) (Math|Float|Lerp (Variables|Default|GetPlayerMaxSpeed) 0.0 (Variables|Default|GetSpeedAlpha)))
        ;[0.15 0.0354 0.03396 0.5] Game Over si trop proche
        (if (<= (Math|Float|Absolute(Float) (Variables|Default|GetPlayerDistance)) (Variables|Settings|GetDeathDistance))
          (Default|FinishGame (Variables|Refs|GetAs%20GI%20Main) false)
          (CallFunction|StopPlayer))))))

(fn ConstructionScript)