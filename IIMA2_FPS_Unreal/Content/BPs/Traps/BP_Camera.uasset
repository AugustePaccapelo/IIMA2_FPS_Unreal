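; Security camera trap that rotates through a looping list of rotations and ends the game as lost when it spots the player.
; The construction script uses trigonometry to fit preview, warning and smaller game-over cones to the spotlight's angle and radius.
; While the player is inside the warning cone, Tick line-traces for obstacles.
; Clear sight recolors light and cone, or calls FinishGame once the dead-zone flag is set.
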(event OnComponentBeginOverlap(ConeWarning)
  (params (OverlappedComponent :type Primitive%20Component%20Object%20Reference) (OtherActor :type Actor%20Object%20Reference) (OtherComp :type Primitive%20Component%20Object%20Reference) (OtherBodyIndex :type Integer) (bFromSweep :type Boolean) (SweepResult :type Hit%20Result%20Structure%20%28by%20ref%29))
  ;[0.15 0.04 0.03506 0.5] Si le joueur est detecté dans l'overlap / sort
  (bind _asbp_player (Utilities|Casting|CastToBP_Player OtherActor))
  (Variables|Refs|SetAs%20BP%20Player _asbp_player)
  (Variables|Default|SetCheckForPlayer true))

(event OnComponentEndOverlap(ConeWarning)
  (params (OverlappedComponent :type Primitive%20Component%20Object%20Reference) (OtherActor :type Actor%20Object%20Reference) (OtherComp :type Primitive%20Component%20Object%20Reference) (OtherBodyIndex :type Integer))
  ;[0.15 0.04 0.03506 0.5] Si le joueur est detecté dans l'overlap / sort
  (Utilities|Casting|CastToBP_Player OtherActor)
  (Variables|Default|SetCheckForPlayer false)
  (Rendering|Components|Light|SetLightColor (Variables|Default|GetSpotLight) (Variables|Colors|GetBasicLightColor) true))

(event OnComponentBeginOverlap(ConeGameOver)
  (params (OverlappedComponent :type Primitive%20Component%20Object%20Reference) (OtherActor :type Actor%20Object%20Reference) (OtherComp :type Primitive%20Component%20Object%20Reference) (OtherBodyIndex :type Integer) (bFromSweep :type Boolean) (SweepResult :type Hit%20Result%20Structure%20%28by%20ref%29))
  ;[0.15 0.0363 0.0401 0.5] Overlap du joueur et sortie de la zone de mort
  (Utilities|Casting|CastToBP_Player OtherActor)
  (Variables|Default|SetIsPlayerInDeadZone true))

(event OnComponentEndOverlap(ConeGameOver)
  (params (OverlappedComponent :type Primitive%20Component%20Object%20Reference) (OtherActor :type Actor%20Object%20Reference) (OtherComp :type Primitive%20Component%20Object%20Reference) (OtherBodyIndex :type Integer))
  ;[0.15 0.0363 0.0401 0.5] Overlap du joueur et sortie de la zone de mort
  (Utilities|Casting|CastToBP_Player OtherActor)
  (Variables|Default|SetIsPlayerInDeadZone true)
  (Rendering|Material|SetMaterial (Variables|Default|GetConePreview) 0 (Variables|Default|GetPreviewMaterial)))

(event Custom|RotateCamera
  (bind _targetrotationsway (Variables|RotationSettings|GetTargetRotationsWay))
  (bind _pivot (Variables|Default|GetPivot))
  (bind _pivot_2 (Variables|Default|GetPivot))
  (bind _returnvalue (Utilities|Array|Length _targetrotationsway))
  (bind _relativerotation (Variables|/Script/Engine.SceneComponent|GetRelativeRotation _pivot))
  ;[0.05695 0.09169 0.15 0.5] Mouvement de la cam
  (if (> _returnvalue 0)
    (if (>= (Variables|Default|GetNextIndex) _returnvalue)
      (Variables|Default|SetNextIndex 0))
    (Components|MoveComponentTo _pivot_2 (Variables|/Script/Engine.SceneComponent|GetRelativeLocation _pivot_2) (Utilities|Array|Get(acopy) (Variables|RotationSettings|GetTargetRotationsWay) (Variables|Default|GetNextIndex)) false false (/ (Math|Float|Max(Float) (Math|Float|Absolute(Float) (- (.Roll (Math|Rotator|BreakRotator (Utilities|Array|Get(acopy) (Variables|RotationSettings|GetTargetRotationsWay) (Variables|Default|GetNextIndex)))) (.roll _relativerotation))) (Math|Float|Absolute(Float) (- (.Pitch (Math|Rotator|BreakRotator (Utilities|Array|Get(acopy) (Variables|RotationSettings|GetTargetRotationsWay) (Variables|Default|GetNextIndex)))) (.pitch _relativerotation))) (Math|Float|Absolute(Float) (- (.Yaw (Math|Rotator|BreakRotator (Utilities|Array|Get(acopy) (Variables|RotationSettings|GetTargetRotationsWay) (Variables|Default|GetNextIndex)))) (.yaw _relativerotation)))) (Variables|RotationSettings|GetRotatingSpeed)) false)
    ;;[0.15 0.04037 0 0.5] wait entre les rotations si y'a l'option
    (if (Variables|RotationSettings|GetWaitBetweenEachRotation)
      (Utilities|FlowControl|Delay (Variables|RotationSettings|GetWaitingTime)))
    ;;[0.02462 0.15 0.03499 0.5] Rapel de la fonction avec le prochain index
    (Math|Integer|IncrementInt (Variables|Default|GetNextIndex)
      (:%20%20
        (CallFunction|RotateCamera)))))

(event Custom|LaunchCameraWarnings
  ;[1 0.8695 0 0.2557] Camera Warnings
  (Rendering|Components|Light|SetLightColor (Variables|Default|GetSpotLight) (Variables|Colors|GetWarningLightColor) true)
  (bind _returnvalue (Rendering|Material|CreateDynamicMaterialInstance (Variables|Default|GetConePreview) 0 (Variables|Default|GetPreviewMaterial) "None" :!class /Script/Engine.PrimitiveComponent))
  (Rendering|Material|SetVectorParameterValue _returnvalue "Emissive Color" (Variables|Colors|GetWarningLightColor) :!class /Script/Engine.MaterialInstanceDynamic)
  (Rendering|Material|SetMaterial (Variables|Default|GetConePreview) 0 _returnvalue))

(event EventBeginPlay
  ;[0.07202 0.09314 0.15 0.5] récupération de la game instance
  (bind _asgi_main (Utilities|Casting|CastToGI_Main (Game|GetGameInstance)))
  (Variables|Refs|SetAs%20GI%20Main _asgi_main)
  (CallFunction|RotateCamera)
  (bind _asbp_player (Utilities|Casting|CastToBP_Player (Game|Player|GetPlayerPawn 0)))
  (Utilities|Array|Add (Variables|Refs|GetActors%20to%20Ignore) _asbp_player)
  (Variables|Default|SetPreviewMaterial (Rendering|Material|GetMaterial (Variables|Default|GetConePreview) 0)))

(event EventTick
  (params (DeltaSeconds :type Float%20%28single-precision%29))
  ;[0.15 0.03509 0.1486 0.5] Si on a detecté le joueur en overlap, on va constamment check si ya un obstacle entre lui et la cam. Si ya plus d'obstacle c'est game over
  (if (Variables|Default|GetCheckForPlayer)
    (bind _hitdetected (CallFunction|CheckforObstacles))
    (if (not _hitdetected)
      (if (Variables|Default|GetIsPlayerInDeadZone)
        (Default|FinishGame (Variables|Refs|GetAs%20GI%20Main) false)
        (else
          (CallFunction|LaunchCameraWarnings))))))

(fn ConstructionScript
  ;[0.3281 0.3081 0.0585 0.5] On met tous nos cones de la meme taille que notre light
  (CallFunction|SetConetoLight 0.0 (Variables|Default|GetConePreview))
  (CallFunction|SetConetoLight 0.0 (Variables|Default|GetConeWarning))
  (CallFunction|SetConetoLight (Variables|Default|GetInnerWarningDistance) (Variables|Default|GetConeGameOver))
  (Rendering|Components|Light|SetLightColor (Variables|Default|GetSpotLight) (Variables|Colors|GetBasicLightColor) true))

(fn SetConetoLight
  (params (Offset :type Float%20%28double-precision%29) (Obj :type Static%20Mesh%20Component%20Object%20Reference))
  (bind _spotlight (Variables|Default|GetSpotLight))
  (bind _spotlight_2 (Variables|Default|GetSpotLight))
  (bind _returnvalue (Transformation|GetWorldRotation _spotlight))
  (bind _attenuationradius (Variables|/Script/Engine.LocalLightComponent|GetAttenuationRadius _spotlight))
  (bind _outerconeangle (Variables|/Script/Engine.SpotLightComponent|GetOuterConeAngle _spotlight))
  (bind _returnvalue_2 (Math|Trig|Tan(Degrees) _outerconeangle))
  (bind _returnvalue_3 (/ _attenuationradius 1e+02))
  (bind _returnvalue_4 (* _returnvalue_2 _returnvalue_3))
  (bind _returnvalue_5 (* _returnvalue_4 2.0))
  (bind _returnvalue_6 (- _returnvalue_5 Offset))
  ;[0.08426 0.1126 0.3198 0.5] On applique la même rotation
  (Transformation|SetWorldRotation Obj (Math|Rotator|MakeRotator (.roll _returnvalue) (+ (.pitch _returnvalue) 9e+01) (.yaw _returnvalue)) false false)
  (Transformation|SetWorldScale3D Obj (Math|Vector|MakeVector _returnvalue_6 _returnvalue_6 _returnvalue_3))
  ;[0.3073 0.1385 0.2844 0.5] On met a la même position (on doit ajuster car pas le mm pivot)
  (Transformation|SetWorldLocation Obj (+ (Transformation|GetWorldLocation _spotlight_2) (* (Math|Vector|GetForwardVector _spotlight_2) (/ (Variables|/Script/Engine.LocalLightComponent|GetAttenuationRadius (Variables|Default|GetSpotLight)) 2.0))) false false))

(fn CheckforObstacles
  (bind _returnvalue (Collision|LineTraceByChannel (Transformation|GetWorldLocation (Variables|Default|GetSpotLight)) (Transformation|GetActorLocation (Variables|Refs|GetAs%20BP%20Player)) "TraceTypeQuery1" false (Variables|Refs|GetActors%20to%20Ignore) "None" true "(R=0.000000,G=1.000000,B=0.912188,A=1.000000)"))
  (return _returnvalue))