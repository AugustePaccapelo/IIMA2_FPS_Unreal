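; Laser trap actor that triggers its room's trap group through GI_Main when the player overlaps the visible beam.
; Line traces up and down find the surfaces within a max length, then the beam is scaled and centered to span between them.
; This fit runs in the construction script and again whenever MoveLaser relocates it.
; It plays a sound on BeginPlay and can be activated or deactivated by toggling its visibility.
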(event OnComponentBeginOverlap(Laser)
  (params (OverlappedComponent :type Primitive%20Component%20Object%20Reference) (OtherActor :type Actor%20Object%20Reference) (OtherComp :type Primitive%20Component%20Object%20Reference) (OtherBodyIndex :type Integer) (bFromSweep :type Boolean) (SweepResult :type Hit%20Result%20Structure%20%28by%20ref%29))
  (bind _as_gi_main (Variables|Default|GetAs%20GI%20Main))
  ;[0.2656 0.06383 0.08397 0.5] Si le joueur est detecté, on déclenche l'effet du piège
  (Utilities|Casting|CastToBP_Player OtherActor)
  (if (not (Variables|/Script/Engine.SceneComponent|GetbHiddenInGame (Variables|Default|GetLaser)))
    (Utilities|IsValid _as_gi_main
      (:Is%20Valid
        (Default|TriggerRoomTraps _as_gi_main (Variables|Default|GetTrapGroup))))))

(event Custom|MoveLaser
  (params (TargetPosition :type Vector))
  ;[0.2797 0.3031 0.1438 0.5] Event a appeler pour bouger le laser (il le bouge et recalcule son render)
  (Transformation|SetWorldLocation (Variables|Default|GetLaser) TargetPosition false false)
  (CallFunction|SetLaserScale))

(event Custom|DeacivateLaser
  ;[0.1768 0.1642 0.2781 0.5] Au cas ou (pour desactiver et reactiver le laser)
  (Development|SetHiddeninGame (Variables|Default|GetLaser) true false))

(event Custom|ActivateLaser
  ;[0.1768 0.1642 0.2781 0.5] Au cas ou (pour desactiver et reactiver le laser)
  (Development|SetHiddeninGame (Variables|Default|GetLaser) false false))

(event EventBeginPlay
  (bind _audio (Variables|Default|GetAudio))
  (bind _asgi_main (Utilities|Casting|CastToGI_Main (Game|GetGameInstance)))
  (Variables|Default|SetAs%20GI%20Main _asgi_main)
  ;[0.2876 0.23 0.5198 0.5] Son des lasers
  (Audio|Components|Audio|SetSound _audio "/Game/Assets/Sounds/Traps/Laser.Laser")
  (Audio|Components|Audio|Play _audio 0.0))

(fn ConstructionScript
  (bind _laser (Variables|Default|GetLaser))
  (bind _lasermaxlenght (Variables|LaserRender|GetlaserMaxLenght))
  (bind _returnvalue (Math|Vector|GetUpVector _laser))
  (bind _returnvalue_2 (/ _lasermaxlenght 2.0))
  (bind _returnvalue_3 (* _returnvalue _returnvalue_2))
  ;[0.2156 0.1226 0.1813 0.5] Point max a atteindre vers le haut et vers le bas
  (Variables|LaserRender|SetlaseMaxUpPoint (+ _returnvalue_3 (Transformation|GetWorldLocation (Variables|Default|GetLaser))))
  (Variables|LaserRender|SetlaseMaxDownPoint (+ (* _returnvalue_3 -1.0) (Transformation|GetWorldLocation (Variables|Default|GetLaser))))
  ;[0.2656 0.2068 0.07534 0.5] Calcul de la taille du laser
  (bind _point (CallFunction|GetLaserHitPoint (Transformation|GetWorldLocation (Variables|Default|GetLaser)) (Variables|LaserRender|GetlaseMaxUpPoint)))
  (Variables|LaserRender|SetupPoint _point)
  (CallFunction|SetLaserScale))

(fn GetLaserHitPoint
  (params (startPoint :type Vector) (maxEndPoint :type Vector))
  (bind (_outhit _returnvalue) (Collision|LineTraceByChannel startPoint maxEndPoint "TraceTypeQuery1" false 0 "None"))
  (if _returnvalue
    (return (.ImpactPoint (Collision|BreakHitResult _outhit)))
    (else
      (return maxEndPoint))))

(fn SetLaserScale
  (bind _laser (Variables|Default|GetLaser))
  (bind _lasermaxlenght (Variables|LaserRender|GetlaserMaxLenght))
  (bind _laser_2 (Variables|Default|GetLaser))
  (bind _returnvalue (Math|Vector|GetUpVector _laser))
  (bind _returnvalue_2 (Transformation|GetWorldScale _laser_2))
  (bind _returnvalue_3 (/ _lasermaxlenght 2.0))
  (bind _returnvalue_4 (* _returnvalue _returnvalue_3))
  ;[0.274 0.1558 0.2304 0.5] Point max a atteindre vers le haut et vers le bas
  (Variables|LaserRender|SetlaseMaxUpPoint (+ _returnvalue_4 (Transformation|GetWorldLocation (Variables|Default|GetLaser))))
  (Variables|LaserRender|SetlaseMaxDownPoint (+ (* _returnvalue_4 -1.0) (Transformation|GetWorldLocation (Variables|Default|GetLaser))))
  ;[0.3073 0.2393 0.08715 0.5] Calcul de la taille du laser
  (bind _point (CallFunction|GetLaserHitPoint (Transformation|GetWorldLocation (Variables|Default|GetLaser)) (Variables|LaserRender|GetlaseMaxUpPoint)))
  (Variables|LaserRender|SetupPoint _point)
  (bind _point_2 (CallFunction|GetLaserHitPoint (- (Variables|LaserRender|GetupPoint) (* (Math|Vector|GetUpVector (Variables|Default|GetLaser)) 0.2)) (Variables|LaserRender|GetlaseMaxDownPoint)))
  (Variables|LaserRender|SetdownPoint _point_2)
  ;[0.1621 0.224 0.0644 0.5] On replace le laser entre les deux points pour que les extrémités touchent bien les deux bords
  (Transformation|SetWorldScale3D _laser_2 (Math|Vector|MakeVector (.x _returnvalue_2) (.y _returnvalue_2) (/ (Math|Vector|Distance(Vector) (Variables|LaserRender|GetupPoint) (Variables|LaserRender|GetdownPoint)) 1e+02)))
  ;[0.08431 0.2115 0.1019 0.5] Calcul de la position du laser (au milieu des deux points)
  (Transformation|SetWorldLocation (Variables|Default|GetLaser) (/ (+ (Variables|LaserRender|GetupPoint) (Variables|LaserRender|GetdownPoint)) 2.0) false true))