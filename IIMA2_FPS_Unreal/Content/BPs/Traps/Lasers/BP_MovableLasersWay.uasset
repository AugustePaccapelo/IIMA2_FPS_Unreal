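; Laser trap that spawns a set number of BP_Laser actors along a spline and moves them back and forth on it.
; BeginPlay places them either stretched evenly over the spline length or at a fixed gap, recording each laser's distance and direction in parallel arrays.
; Tick advances each distance by speed and direction, clamps and reverses it at the spline ends, then passes the new world location to MoveLaser.
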(event EventTick
  (params (DeltaSeconds :type Float%20%28single-precision%29))
  (bind _spline (Variables|Default|GetSpline))
  (bind _returnvalue (Spline|GetSplineLength _spline))
  ;[0 0.1145 0.15 0.5] Mouvement des lasers
  (for (_array_element _array_index) (Variables|Default|GetLasers)
    ;[0.009821 0.15 0.1354 0.5] Calcule de la nouvelle distance target du laser selon la speed et sa distance actuelle (et sa direction)
    (bind _output_get (Variables|Default|SetNewDistance (+ (Utilities|Array|Get(acopy) (Variables|Movement|GetLaserDistance) _array_index) (* DeltaSeconds (Variables|Movement|GetlaserSpeed) (Utilities|Array|Get(acopy) (Variables|Movement|GetLaserDirectionsForward) _array_index)))))
    ;[0.15 0.08152 0.1388 0.5] Si la distance target dépasse la longeur de la spline, le laser doit passer au retour (il a fini l'allée)
    (if (>= _output_get _returnvalue)
      (Variables|Default|SetNewDistance _returnvalue)
      (Utilities|Array|SetArrayElem (Variables|Movement|GetLaserDirectionsForward) _array_index -1)
      (else
        ;[0.15 0.09612 0.04203 0.5] Si la distance est inférieur à 0, le laser a fini le retour et repasse à l'allée
        (if (<= (Variables|Default|GetNewDistance) 0.0)
          (Variables|Default|SetNewDistance 0.0)
          (Utilities|Array|SetArrayElem (Variables|Movement|GetLaserDirectionsForward) _array_index 1))))
    ;[0.07606 0.15 0.1063 0.5] set de la nouvelle distance clamp
    (Utilities|Array|SetArrayElem (Variables|Movement|GetLaserDistance) _array_index (Variables|Default|GetNewDistance))
    ;[0.15 0.08538 0.142 0.5] calcule de la nouvelle position et mouvement
    (Default|MoveLaser _array_element (Spline|GetLocationatDistanceAlongSpline (Variables|Default|GetSpline) (Variables|Default|GetNewDistance) "World"))))

(event EventBeginPlay
  (bind _lasersnumber (Variables|Placement|GetlasersNumber))
  (bind _returnvalue (- _lasersnumber 1))
  (for _index (range 0 _returnvalue)
    (if (Variables|Placement|GetStrechLaserOnSpline)
      (Variables|Placement|SetSpawnTransform (Spline|GetTransformatDistanceAlongSpline (Variables|Default|GetSpline) (Math|Conversions|ToFloat(Integer) (* _index (/ (Spline|GetSplineLength (Variables|Default|GetSpline)) _returnvalue))) "World" false))
      (Variables|Default|SetcurrentLaserDistance (Math|Conversions|ToFloat(Integer) (* _index (/ (Spline|GetSplineLength (Variables|Default|GetSpline)) _returnvalue))))
      (else
        (Variables|Placement|SetSpawnTransform (Spline|GetTransformatDistanceAlongSpline (Variables|Default|GetSpline) (* _index (Variables|Placement|GetLaserGap)) "World" false))
        (Variables|Default|SetcurrentLaserDistance (* _index (Variables|Placement|GetLaserGap)))))
    ;[0.15 0.03952 0.136 0.5] Spawn du bon type de laser
    (bind _returnvalue_2 (Game|SpawnActorfromClass "/Game/BPs/Traps/Lasers/BP_Laser.BP_Laser_C" (Variables|Placement|GetSpawnTransform) "Undefined" "MultiplyWithRoot" 0 0))
    (Utilities|Array|Add (Variables|Default|GetLasers) _returnvalue_2)
    ;[0.01402 0.15 0.1148 0.5] Set up de la distance de départ du laser
    (Utilities|Array|Add (Variables|Movement|GetLaserDistance) (Variables|Default|GetcurrentLaserDistance))
    ;[0.15 0.06835 0.06003 0.5] Initialisation de la direction du laser (1 pour allée et -1 pour retour pour multipliser la distance plus tard)
    (Utilities|Array|Add (Variables|Movement|GetLaserDirectionsForward) 1)))

(fn ConstructionScript)