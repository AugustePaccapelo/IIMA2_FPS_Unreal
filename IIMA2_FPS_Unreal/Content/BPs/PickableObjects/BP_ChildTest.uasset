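; BP_ChildTest is a test child Blueprint of an interactable pickable object that the player can collect.
; On interaction it casts player controller 0 to PC_Player, passes itself to AddToInventory, prints a debug message and destroys the actor.
; The hover and unhover events are empty, and the construction script only calls the parent.
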(event EventBeginPlay
  (|CallParentFunction) ; This node is disabled and will not be called.\nDrag off pins to build functionality.
)

(event Collision|EventActorBeginOverlap
  (params (OtherActor :type Actor%20Object%20Reference))
  (|CallParentFunction OtherActor) ; This node is disabled and will not be called.\nDrag off pins to build functionality.
)

(event EventTick
  (params (DeltaSeconds :type Float%20%28single-precision%29))
  (|CallParentFunction DeltaSeconds) ; This node is disabled and will not be called.\nDrag off pins to build functionality.
)

(event EventOnHover)

(event EventOnInteracte
  (bind _aspc_player (Utilities|Casting|CastToPC_Player (Game|GetPlayerController 0)))
  (Default|AddtoInventory _aspc_player self)
  (Development|PrintString "Hello")
  (Actor|DestroyActor))

(event EventUnHover)

(fn ConstructionScript
  (|CallParentFunction))