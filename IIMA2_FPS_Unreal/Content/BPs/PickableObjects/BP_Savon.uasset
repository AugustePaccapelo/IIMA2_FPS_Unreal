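; BP_Savon is a pickable soap that stuns enemy characters on contact.
; When its collision sphere overlaps a Chara_Enemy, it triggers that enemy's stun, plays a soap sound, starts the spawner's respawn timer and destroys itself.
; Sphere hits spawn a soap decal actor at the impact point, and hover events toggle a highlight overlay material on the mesh.
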(event OnComponentBeginOverlap(CollisionSphere)
  (params (OverlappedComponent :type Primitive%20Component%20Object%20Reference) (OtherActor :type Actor%20Object%20Reference) (OtherComp :type Primitive%20Component%20Object%20Reference) (OtherBodyIndex :type Integer) (bFromSweep :type Boolean) (SweepResult :type Hit%20Result%20Structure%20%28by%20ref%29))
  (if (== (Utilities|GetClass OtherActor) "/Game/BPs/AI/Chara_Enemy.Chara_Enemy_C")
    (bind _aschara_enemy (Utilities|Casting|CastToChara_Enemy OtherActor))
    (Default|CEStun _aschara_enemy (Variables|Default|GetStunDuration))
    (Audio|SpawnSoundatLocation "/Game/Assets/Sounds/MetaSounds/MSS_Soap.MSS_Soap" (Transformation|GetActorLocation) "0, 0, 0" 1.0 1.0 0.0 0 0)
    (CallFunction|StartSpawnerRespawnTimer)
    (Actor|DestroyActor)))

(event OnComponentHit(CollisionSphere)
  (params (HitComponent :type Primitive%20Component%20Object%20Reference) (OtherActor :type Actor%20Object%20Reference) (OtherComp :type Primitive%20Component%20Object%20Reference) (NormalImpulse :type Vector :default "0, 0, 0") (Hit :type Hit%20Result%20Structure%20%28by%20ref%29))
  (Game|SpawnActorfromClass "/Game/BPs/PickableObjects/BP_DecalSoapHit.BP_DecalSoapHit_C" (Math|Transform|MakeTransform (.ImpactPoint (Collision|BreakHitResult Hit)) "0, 0, 0" "1.000000,1.000000,1.000000") "Undefined" "MultiplyWithRoot" 0 0))

(event EventBeginPlay
  (|CallParentFunction) ; This node is disabled and will not be called.\nDrag off pins to build functionality.
)

(event Collision|EventActorBeginOverlap
  (params (OtherActor :type Actor%20Object%20Reference))
  (|CallParentFunction OtherActor) ; This node is disabled and will not be called.\nDrag off pins to build functionality.
)

(event EventTick
  (params (DeltaSeconds :type Float%20%28single-precision%29))
  (|CallParentFunction DeltaSeconds) ; This node is disabled and will not be called.\nDrag off pins to build functionality.
)

(event EventUnHover
  (Rendering|Material|SetOverlayMaterial (Variables|Default|GetSM) 0 :!class /Script/Engine.MeshComponent))

(event EventOnHover
  (Rendering|Material|SetOverlayMaterial (Variables|Default|GetSM) (Variables|Default|GetHoverMaterial) :!class /Script/Engine.MeshComponent))

(fn ConstructionScript
  (|CallParentFunction))