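; Single-use pickable raygun that kills the enemy in the player's line of fire and knocks the player back.
; UseItem toggles charging; Tick feeds loading particles and fires automatically at full charge, with charge sound pitch scaled to charge time.
; Firing reports noise, line-traces forward from the player and draws a Niagara beam.
; The spent gun leaves the hand, starts its spawner respawn timer and self-destroys after a delay.
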(event Custom|proxy_NEShootFinished
  ;[0.15 0.15 0.15 0.5] Shoot
  ;;[0.15 0.15 0.15 0.5] Destroy the raygun after 5 sec
  (Utilities|Time|ClearandInvalidateTimerbyHandle (Variables|Raygun|GetSelfDeathTimer))
  (Actor|DestroyActor))

(event Custom|CE_Shoot
  (bind _returnvalue (Transformation|GetActorLocation))
  ;[0.15 0.15 0.15 0.5] Shoot
  (Class|AISenseHearing|ReportNoiseEvent (Transformation|GetActorLocation) (Variables|Raygun|GetLoudness) self (Variables|Raygun|GetmaxSoundRange) "None")
  ;;[0.15 0.15 0.15 0.5] Play shot sound
  (Audio|SpawnSoundatLocation "/Game/Assets/Sounds/MetaSounds/MSS_RaygunShot.MSS_RaygunShot" _returnvalue "0, 0, 0" 2.0 1.0 0.0 "/Game/Assets/Sounds/SA_Distance.SA_Distance" 0)
  ;;[0.15 0.15 0.15 0.5] Sound particule
  (Niagara|SpawnSystematLocation "/Game/Assets/Particules/NS_SoundCue.NS_SoundCue" _returnvalue)
  (Variables|Raygun|SetDidShot true)
  (bind _outhit (Utilities|ShootLineTrace))
  (Variables|Raygun|SetHitActor (.HitActor (Collision|BreakHitResult _outhit)))
  ;;[0.15 0.15 0.15 0.5] Start Niagara System Shoot
  (Class|NiagaraComponent|SetVariablePosition (Variables|Default|GetNS_RaygunShoot) (Variables|Raygun|GetEndPosName) (.ImpactPoint (Collision|BreakHitResult _outhit)))
  (Class|NiagaraComponent|SetVariablePosition (Variables|Default|GetNS_RaygunShoot) (Variables|Raygun|GetStartPosName) (Transformation|GetWorldLocation (Variables|Default|GetCanon)))
  (Components|Activation|Activate (Variables|Default|GetNS_RaygunShoot) false)
  ;;[0.15 0.15 0.15 0.5] Stop loading particules
  (Niagara|SetNiagaraVariable(Float) (Variables|Default|GetNS_RaygunLoading) (Variables|Raygun|GetSpawnRageName) 0.0)
  ;;[0.15 0.15 0.15 0.5] Hide the raygun
  (Rendering|SetVisibility (Variables|Default|GetRenderer) false true)
  ;;[0.15 0.15 0.15 0.5] Destroy the raygun after 5 sec
  (bind _returnvalue_2 (Utilities|Time|SetTimerbyEvent (delegate Custom|proxy_NEShootFinished) 5.0))
  (Variables|Raygun|SetSelfDeathTimer _returnvalue_2)
  ;;[0.15 0.15 0.15 0.5] Remove raygun from inventory
  (bind _asbp_player (Utilities|Casting|CastToBP_Player (Game|Player|GetPlayerPawn 0)))
  (Default|RemoveItemfromHand _asbp_player)
  (Rendering|SetActorHiddenInGame false)
  (CallFunction|StartSpawnerRespawnTimer)
  ;;[0.15 0.15 0.15 0.5] Apply knock back
  (Default|AddVelocity _asbp_player (* (Transformation|GetActorForwardVector _asbp_player) (Variables|Raygun|GetRaygunKnockbackForce) -1.0))
  ;;[0.15 0.15 0.15 0.5] If hited an enemy, kill it
  (if (== (Utilities|GetClass (Variables|Raygun|GetHitActor)) "/Game/BPs/AI/Chara_Enemy.Chara_Enemy_C")
    (Niagara|SpawnSystematLocation 0 (Transformation|GetActorLocation (Variables|Raygun|GetHitActor)))
    (bind _aschara_enemy (Utilities|Casting|CastToChara_Enemy (Variables|Raygun|GetHitActor)))
    (Default|DisableActor _aschara_enemy)))

(event EventBeginPlay
  ;[0.15 0.15 0.15 0.5] BeginPlay
  (Variables|Default|SetMesh (Variables|Default|GetStaticMesh))
  (|CallParentFunction)
  (bind _returnvalue (Audio|SpawnSoundAttached "/Game/Assets/Sounds/MetaSounds/MSS_RaygunCharge.MSS_RaygunCharge" (Variables|Transformation|GetRootComponent) "None" "0, 0, 0" "0, 0, 0" "KeepRelativeOffset" false 1.5 (/ (Variables|Default|GetChargeSoundBaseDuration) (Variables|Raygun|GetChargeTime)) 0.0 0 0 false))
  (bind _output_get (Variables|Default|SetSC_Charge _returnvalue))
  (Audio|Components|Audio|Stop _output_get))

(event EventTick
  (params (DeltaSeconds :type Float%20%28single-precision%29))
  ;[0.15 0.15 0.15 0.5] Charging
  (|CallParentFunction DeltaSeconds)
  ;;[0.15 0.15 0.15 0.5] If is not charging or has shoot, return
  (if (and (Variables|Raygun|GetIsCharging) (not (Variables|Raygun|GetDidShot)))
    ;;[0.15 0.15 0.15 0.5] Update current charge
    (bind _output_get (Variables|Raygun|SetCurrentCharge (+ (Variables|Raygun|GetCurrentCharge) DeltaSeconds)))
    ;;[0.15 0.15 0.15 0.5] Update niagara Loading
    (Niagara|SetNiagaraVariable(Float) (Variables|Default|GetNS_RaygunLoading) (Variables|Raygun|GetSpawnRageName) (/ _output_get (Variables|Raygun|GetChargeTime)))
    ;;[0.15 0.15 0.15 0.5] If charge is complete, shoot
    (if (>= (Variables|Raygun|GetCurrentCharge) (Variables|Raygun|GetChargeTime))
      (CallFunction|CEShoot))))

(fn ConstructionScript
  (|CallParentFunction))

(fn UseItem
  (params (Player :type Actor%20Object%20Reference))
  (|CallParentFunction Player)
  (Variables|Raygun|SetIsCharging (not (Variables|Raygun|GetIsCharging)))
  (Variables|Raygun|SetCurrentCharge 0.0)
  (Niagara|SetNiagaraVariable(Float) (Variables|Default|GetNS_RaygunLoading) (Variables|Raygun|GetSpawnRageName) 0.0)
  (if (Variables|Raygun|GetIsCharging)
    (Audio|Components|Audio|Play (Variables|Default|GetSC_Charge) 0.0)
    (else
      (Audio|Components|Audio|Stop (Variables|Default|GetSC_Charge)))))