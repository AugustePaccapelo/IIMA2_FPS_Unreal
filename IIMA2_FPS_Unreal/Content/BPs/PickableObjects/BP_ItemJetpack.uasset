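; BP_ItemJetpack is a pickable item that unlocks the jetpack for the player when interacted with.
; On interaction it calls UnlockJetpack on the PC_Player player controller, then destroys itself.
; Each tick it bobs around its starting location using a sine oscillation with configurable speed, range and direction.
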(event EventBeginPlay
  (|CallParentFunction)
  (Variables|Default|SetStartMeshLoc (Transformation|GetActorLocation)))

(event Collision|EventActorBeginOverlap
  (params (OtherActor :type Actor%20Object%20Reference))
  (|CallParentFunction OtherActor) ; This node is disabled and will not be called.\nDrag off pins to build functionality.
)

(event EventTick
  (params (DeltaSeconds :type Float%20%28single-precision%29))
  (|CallParentFunction DeltaSeconds)
  (Utilities|FloatingAnimation))

(event EventOnInteracte
  (bind _aspc_player (Utilities|Casting|CastToPC_Player (Game|GetPlayerController 0)))
  (Default|UnlockJetpack _aspc_player)
  (Actor|DestroyActor))

(fn ConstructionScript
  (|CallParentFunction))