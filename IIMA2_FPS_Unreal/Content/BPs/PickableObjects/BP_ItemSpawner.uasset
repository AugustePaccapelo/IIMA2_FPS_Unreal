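; BP_ItemSpawner is an actor that spawns a chosen item class at its own transform on BeginPlay and can respawn it after a delay.
; CreateItem hands each spawned item a reference to its spawner.
; StartRespawnTimer sets a timer for SpawnItem, which recreates the item, has GI_Main respawn the listed enemy groups, then clears the timer.
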(event Custom|StartRespawnTimer
  (bind _returnvalue (Utilities|Time|SetTimerbyEvent (delegate Custom|SpawnItem) (Variables|Default|GetSpawningTime))))

(event Custom|SpawnItem
  (Utilities|CreateItem)
  (for _array_element (Variables|Default|GetEnemyGroupToSpawn)
    (Default|RespawnEnemyGroup (Variables|Default|GetGIMain) _array_element))
  (Utilities|Time|ClearandInvalidateTimerbyHandle (stale Custom|StartRespawnTimer _returnvalue)))

(event EventBeginPlay
  (Utilities|CreateItem)
  (bind _asgi_main (Utilities|Casting|CastToGI_Main (Game|GetGameInstance)))
  (Variables|Default|SetGIMain _asgi_main))

(event Collision|EventActorBeginOverlap
  (params (OtherActor :type Actor%20Object%20Reference)))

(event EventTick
  (params (DeltaSeconds :type Float%20%28single-precision%29)))

(fn ConstructionScript)