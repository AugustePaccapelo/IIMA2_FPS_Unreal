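; BP_ChildTestCube is a test pickable object, a child Blueprint that overrides its parent's hover, interact, equip and use hooks.
; Hover toggles a highlight by setting or clearing an overlay material on the Cube mesh.
; Interaction defers to the parent, while equip and unequip only print French debug messages.
; UseItem is overridden empty, with the parent call left unconnected, so using the cube does nothing.
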(event EventBeginPlay
  (|CallParentFunction))

(event Collision|EventActorBeginOverlap
  (params (OtherActor :type Actor%20Object%20Reference))
  (|CallParentFunction OtherActor) ; This node is disabled and will not be called.\nDrag off pins to build functionality.
)

(event EventTick
  (params (DeltaSeconds :type Float%20%28single-precision%29))
  (|CallParentFunction DeltaSeconds) ; This node is disabled and will not be called.\nDrag off pins to build functionality.
)

(event EventOnHover
  (Rendering|Material|SetOverlayMaterial (Variables|Default|GetCube) (Variables|Default|GetHoverMaterial) :!class /Script/Engine.MeshComponent))

(event EventOnEquipe
  (Development|PrintString "Je  suis équpé"))

(event EventUnHover
  (Rendering|Material|SetOverlayMaterial (Variables|Default|GetCube) 0 :!class /Script/Engine.MeshComponent))

(event EventUnEquipe
  (Development|PrintString "Je  suis plus équpé"))

(event EventOnInteracte
  (|CallParentFunction))

(fn ConstructionScript
  (|CallParentFunction))

(fn UseItem
  (params (Player :type Actor%20Object%20Reference)))