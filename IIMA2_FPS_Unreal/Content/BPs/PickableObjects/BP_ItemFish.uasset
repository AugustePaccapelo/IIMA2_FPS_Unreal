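; Pickable fish item that can be thrown as a noisemaker or eaten from the player's hand, built on a parent item class.
; After a throw, impact starts looping noise bursts (AI noise event, sound, Niagara cue) and a death timer, with a fallback auto-death timer.
; Re-equipping clears the impact timers.
; Eating makes noise instigated by the player; eating and both deaths start spawner respawn before destroying the fish.
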(event OnComponentHit(CollisionSphere)
  (params (HitComponent :type Primitive%20Component%20Object%20Reference) (OtherActor :type Actor%20Object%20Reference) (OtherComp :type Primitive%20Component%20Object%20Reference) (NormalImpulse :type Vector :default "0, 0, 0") (Hit :type Hit%20Result%20Structure%20%28by%20ref%29))
  (if (Variables|Default|GetIsThrown)
    (Utilities|FlowControl|Sequence
      (:then_0
        (bind _returnvalue (Utilities|Time|SetTimerbyEvent (delegate Custom|ProxyMakeFishNoisesOnHit) (Variables|Default|GetTimeBetweenNoises) true true))
        (bind _returnvalue_2 (Utilities|Time|SetTimerbyEvent (delegate Custom|Death) (Variables|Default|GetLifeSpan2) false true)))
      (:then_1
        (Utilities|FlowControl|DoOnce false
          (:Completed
            (CallFunction|MakeFishNoises)))))))

(event Custom|ProxyMakeFishNoises
  (if (Variables|Default|GetIsHeld)
    (CallFunction|MakeFishNoises)))

(event Custom|MakeFishNoises
  (bind _returnvalue (Transformation|GetActorLocation))
  (Class|AISenseHearing|ReportNoiseEvent _returnvalue (Variables|Default|GetNoiseLoudness) self (Variables|Default|GetNoiseRange) "None")
  (Audio|SpawnSoundatLocation "/Game/Assets/Sounds/MetaSounds/MSS_FISHHeld.MSS_FISHHeld" _returnvalue "0, 0, 0" (Variables|Default|GetNoiseVolumeMultiplier) 1.0 0.0 "/Game/Assets/Sounds/SA_Distance.SA_Distance" 0)
  (Niagara|SpawnSystematLocation "/Game/Assets/Particules/NS_SoundCue.NS_SoundCue" _returnvalue))

(event Custom|ProxyMakeFishNoisesOnHit
  (CallFunction|MakeFishNoises))

(event Custom|EatFish
  (bind _returnvalue (Transformation|GetActorLocation))
  (Class|AISenseHearing|ReportNoiseEvent _returnvalue (Variables|Default|GetNoiseLoudness) (Game|Player|GetPlayerPawn 0) (Variables|Default|GetNoiseRange) "None")
  (Audio|SpawnSoundatLocation "/Game/Assets/Sounds/MetaSounds/MSS_FISHEaten.MSS_FISHEaten" _returnvalue "0, 0, 0" (Variables|Default|GetNoiseVolumeMultiplier) 1.0 0.0 "/Game/Assets/Sounds/SA_Distance.SA_Distance" 0)
  (CallFunction|StartSpawnerRespawnTimer)
  (Niagara|SpawnSystematLocation "/Game/Assets/Particules/NS_SoundCue.NS_SoundCue" _returnvalue)
  (Actor|DestroyActor))

(event Custom|Death
  (CallFunction|StartSpawnerRespawnTimer)
  (Actor|DestroyActor))

(event Custom|proxy_AutoDeath
  (Utilities|Time|ClearandInvalidateTimerbyHandle (stale EventOnThrow _returnvalue))
  (CallFunction|StartSpawnerRespawnTimer)
  (Actor|DestroyActor))

(event Custom|OnDestroyed_Event
  (params (DestroyedActor :type Actor%20Object%20Reference))
  (Development|PrintString "Fish Destroyed"))

(event Custom|OnEndPlay_Event
  (params (Actor :type Actor%20Object%20Reference) (EndPlayReason :type EEndPlayReason%20Enum :default "Destroyed")))

(event EventBeginPlay
  (Variables|Default|SetMesh (Variables|Default|GetFishMesh))
  (|CallParentFunction))

(event Collision|EventActorBeginOverlap
  (params (OtherActor :type Actor%20Object%20Reference))
  (|CallParentFunction OtherActor) ; This node is disabled and will not be called.\nDrag off pins to build functionality.
)

(event EventTick
  (params (DeltaSeconds :type Float%20%28single-precision%29))
  (|CallParentFunction DeltaSeconds))

(event EventOnInteracte
  (|CallParentFunction)
  (Variables|Default|SetIsThrown false))

(event EventOnEquipe
  (|CallParentFunction)
  (Variables|Default|SetOscillationSpeed 0.0)
  (Variables|/Script/Engine.RotatingMovementComponent|SetRotationRate (Variables|Default|GetRotatingMovement) "0, 0, 0")
  (Variables|Default|SetIsThrown false)
  (Utilities|Time|ClearandInvalidateTimerbyHandle (stale OnComponentHit(CollisionSphere) _returnvalue))
  (Utilities|Time|ClearandInvalidateTimerbyHandle (stale OnComponentHit(CollisionSphere) _returnvalue_2)))

(event EventUnEquipe)

(event EventOnThrow
  (|CallParentFunction)
  (Variables|Default|SetIsThrown true)
  (Utilities|FlowControl|Sequence
    (:then_0
      (Utilities|FlowControl|DoOnce false) ; enters at Reset
    )
    (:then_1
      (bind _returnvalue (Utilities|Time|SetTimerbyEvent (delegate Custom|proxy_AutoDeath) 2e+01)))))

(fn ConstructionScript)

(fn UseItem
  (params (Player :type Actor%20Object%20Reference))
  (|CallParentFunction 0)
  (bind _asbp_player (Utilities|Casting|CastToBP_Player (Game|Player|GetPlayerPawn 0)))
  (Default|RemoveItemfromHand _asbp_player)
  (CallFunction|EatFish))