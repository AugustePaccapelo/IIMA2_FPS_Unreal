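; BP_LaunchInfosBox is a trigger box that shows an explanation info box when the player enters it.
; On BeginPlay it caches the game HUD and the GI_Main game instance.
; When BP_Player overlaps the box, it passes ExplanationDataRowName to the HUD for display, records it uniquely in the game instance's UnlockedTutos, then calls DestroyTutos with that row name.
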(event OnComponentBeginOverlap(Box)
  (params (OverlappedComponent :type Primitive%20Component%20Object%20Reference) (OtherActor :type Actor%20Object%20Reference) (OtherComp :type Primitive%20Component%20Object%20Reference) (OtherBodyIndex :type Integer) (bFromSweep :type Boolean) (SweepResult :type Hit%20Result%20Structure%20%28by%20ref%29))
  (Utilities|Casting|CastToBP_Player OtherActor)
  (Default|DisplayInfosBox (Variables|Default|GetAs%20HUD%20Game) (Variables|Default|GetExplanationDataRowName))
  (Utilities|Array|AddUnique (Variables|/Game/BPs/GI_Main.GI_Main_C|GetUnlockedTutos (Variables|Default|GetAs%20GI%20Main)) (Variables|Default|GetExplanationDataRowName))
  (Default|DestroyTutos (Variables|Default|GetAs%20GI%20Main) (Variables|Default|GetExplanationDataRowName)))

(event EventBeginPlay
  (bind _ashud_game (Utilities|Casting|CastToHUD_Game (HUD|GetHUD (Game|GetPlayerController 0))))
  (Variables|Default|SetAs%20HUD%20Game _ashud_game)
  (bind _asgi_main (Utilities|Casting|CastToGI_Main (Game|GetGameInstance)))
  (Variables|Default|SetAs%20GI%20Main _asgi_main))

(fn ConstructionScript)