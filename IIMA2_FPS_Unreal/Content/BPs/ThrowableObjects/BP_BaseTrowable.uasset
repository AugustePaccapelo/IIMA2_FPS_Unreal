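; Base throwable actor that, as shown here, only visualizes a predicted throw arc and has no runtime logic.
; The construction script predicts a projectile path from the actor's location along its forward vector scaled by TrowForce, then feeds it into the Spline.
; AddSplineMeshs adds a Z-forward spline mesh for each segment longer than MinDistance, shaped by the spline's points and tangents.
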(event EventBeginPlay)

(event Collision|EventActorBeginOverlap
  (params (OtherActor :type Actor%20Object%20Reference)))

(event EventTick
  (params (DeltaSeconds :type Float%20%28single-precision%29)))

(fn ConstructionScript
  (bind _outpathpositions (Class|GameplayStatics|BlueprintPredictProjectilePathbyTraceChannel (Transformation|GetActorLocation) (* (Transformation|GetActorForwardVector) (Variables|Default|GetTrowForce)) true 5e+01 "ECC_WorldDynamic" false 0 "ForOneFrame" 0.0 1e+01 3.0))
  (Spline|SetSplinePoints (Variables|Default|GetSpline) _outpathpositions "World" true)
  (CallFunction|AddSplineMeshs))

(fn AddSplineMeshs
  (bind _spline (Variables|Default|GetSpline))
  (bind _spline_2 (Variables|Default|GetSpline))
  (for _index (range 0 (- (Spline|GetNumberOfSplinePoints (Variables|Default|GetSpline)) 2))
    (if (> (- (Spline|GetDistanceAlongSplineatSplinePoint _spline_2 (+ _index 1)) (Spline|GetDistanceAlongSplineatSplinePoint _spline_2 _index)) (Variables|Default|GetMinDistance))
      (bind _returnvalue (AddComponent|AddSplineMeshComponent false))
      (bind _output_get (LocalVariables|SetSSMC _returnvalue))
      (Components|StaticMesh|SetStaticMesh _output_get (Variables|Default|GetMesh))
      (SplineMesh|SetStartandEnd (LocalVariables|GetSSMC) (.Location (Spline|GetLocationandTangentatSplinePoint _spline _index "Local")) (.Tangent (Spline|GetLocationandTangentatSplinePoint _spline _index "Local")) (.Location (Spline|GetLocationandTangentatSplinePoint _spline (+ _index 1) "Local")) (.Tangent (Spline|GetLocationandTangentatSplinePoint _spline (+ _index 1) "Local")) true :!class /Script/Engine.SplineMeshComponent)
      (SplineMesh|SetForwardAxis (LocalVariables|GetSSMC) "Z" false)
      (SplineMesh|SetStartScale (LocalVariables|GetSSMC) "(X=1.000000,Y=1.000000)" false :!class /Script/Engine.SplineMeshComponent)
      (SplineMesh|SetEndScale (LocalVariables|GetSSMC) "(X=1.000000,Y=1.000000)" false :!class /Script/Engine.SplineMeshComponent))))