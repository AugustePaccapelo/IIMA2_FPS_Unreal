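; BP_Checkpoint is a checkpoint actor that saves the player's respawn transform when the player touches it.
; ActorBeginOverlap casts and caches the GI_Main game instance.
; When the Trigger component's overlapping actor matches the BP_Player reference, it writes PlayerTransform's world transform to the game instance's RespawnTransform.
; Debug prints report either the save or the name of any other overlapping actor.
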(event OnComponentBeginOverlap(Trigger)
  (params (OverlappedComponent :type Primitive%20Component%20Object%20Reference) (OtherActor :type Actor%20Object%20Reference) (OtherComp :type Primitive%20Component%20Object%20Reference) (OtherBodyIndex :type Integer) (bFromSweep :type Boolean) (SweepResult :type Hit%20Result%20Structure%20%28by%20ref%29))
  (if (== OtherActor "/Game/BPs/BP_Player.BP_Player")
    (Variables|/Game/BPs/GI_Main.GI_Main_C|SetRespawnTransform (Variables|Default|GetGameInstance) (Transformation|GetWorldTransform (Variables|Default|GetPlayerTransform)))
    (Development|PrintString "YYOHO")
    (else
      (Development|PrintString (Utilities|GetObjectName OtherActor)))))

(event EventBeginPlay)

(event Collision|EventActorBeginOverlap
  (params (OtherActor :type Actor%20Object%20Reference))
  (bind _asgi_main (Utilities|Casting|CastToGI_Main (Game|GetGameInstance)))
  (Variables|Default|SetGameInstance _asgi_main))

(event EventTick
  (params (DeltaSeconds :type Float%20%28single-precision%29)))

(fn ConstructionScript)