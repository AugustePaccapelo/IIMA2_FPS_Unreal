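; An obsolete player Blueprint, going by its name, that provides six-degree-of-freedom thruster flight through Enhanced Input.
; Forward, strafe and elevation inputs add forces to BoxPhysic along the actor's axes, scaled by ThrusterSpeed.
; Look and rotation inputs directly apply local pitch, yaw and roll rather than torque.
; Braking applies force against velocity and zeroes it below a small speed threshold; brake-combo events are empty.
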(event Input|EnhancedActionEvents|EnhancedInputActionIA_Braking
  (params (ActionValue :type Boolean) (ElapsedSeconds :type Float%20%28double-precision%29) (TriggeredSeconds :type Float%20%28double-precision%29) (InputAction :type Input%20Action%20Object%20Reference :default "/Game/Inputs/InputActions/IA_Braking.IA_Braking"))
  (bind _returnvalue (Transformation|GetVelocity))
  (bind _returnvalue_2 (Math|Vector|VectorLengthSquared _returnvalue))
  (Development|PrintString (Utilities|String|ToString(Float) _returnvalue_2))
  (if (> 1e+03 _returnvalue_2)
    (Physics|SetPhysicsLinearVelocity (Variables|Default|GetBoxPhysic) "0, 0, 0" false "None")
    (else
      (Physics|AddForce (Variables|Default|GetBoxPhysic) (* (* (Math|Vector|Normalize _returnvalue) (Variables|Default|GetBreakingForce)) -1.0) "None" false))))

(event Input|EnhancedActionEvents|EnhancedInputActionIA_Forward
  (params (ActionValue :type Float%20%28double-precision%29) (ElapsedSeconds :type Float%20%28double-precision%29) (TriggeredSeconds :type Float%20%28double-precision%29) (InputAction :type Input%20Action%20Object%20Reference :default "/Game/Inputs/InputActions/IA_Forward.IA_Forward"))
  (Physics|AddForce (Variables|Default|GetBoxPhysic) (* (* (Transformation|GetActorForwardVector) ActionValue) (Variables|Default|GetThrusterSpeed)) "None" false))

(event Input|EnhancedActionEvents|EnhancedInputActionIA_BrakeComboLeft
  (params (ActionValue :type Boolean) (ElapsedSeconds :type Float%20%28double-precision%29) (TriggeredSeconds :type Float%20%28double-precision%29) (InputAction :type Input%20Action%20Object%20Reference :default "/Game/Inputs/InputActions/IA_BrakeComboLeft.IA_BrakeComboLeft")))

(event Input|EnhancedActionEvents|EnhancedInputActionIA_Strafe
  (params (ActionValue :type Float%20%28double-precision%29) (ElapsedSeconds :type Float%20%28double-precision%29) (TriggeredSeconds :type Float%20%28double-precision%29) (InputAction :type Input%20Action%20Object%20Reference :default "/Game/Inputs/InputActions/IA_Strafe.IA_Strafe"))
  (Physics|AddForce (Variables|Default|GetBoxPhysic) (* (* (Transformation|GetActorRightVector) ActionValue) (Variables|Default|GetThrusterSpeed)) "None" false))

(event Input|EnhancedActionEvents|EnhancedInputActionIA_Elevation
  (params (ActionValue :type Float%20%28double-precision%29) (ElapsedSeconds :type Float%20%28double-precision%29) (TriggeredSeconds :type Float%20%28double-precision%29) (InputAction :type Input%20Action%20Object%20Reference :default "/Game/Inputs/InputActions/IA_Elevation.IA_Elevation"))
  (Physics|AddForce (Variables|Default|GetBoxPhysic) (* (* (Transformation|GetActorUpVector) ActionValue) (Variables|Default|GetThrusterSpeed)) "None" false))

(event Input|EnhancedActionEvents|EnhancedInputActionIA_Look
  (params (ActionValue :type Vector%202D%20Structure) (ElapsedSeconds :type Float%20%28double-precision%29) (TriggeredSeconds :type Float%20%28double-precision%29) (InputAction :type Input%20Action%20Object%20Reference :default "/Game/Inputs/InputActions/IA_Look.IA_Look"))
  (Transformation|AddActorLocalRotation (Math|Rotator|MakeRotator 0.0 (* (.y ActionValue) 1.0) (* (.x ActionValue) 1.0)) false false))

(event Input|EnhancedActionEvents|EnhancedInputActionIA_Rotation
  (params (ActionValue :type Float%20%28double-precision%29) (ElapsedSeconds :type Float%20%28double-precision%29) (TriggeredSeconds :type Float%20%28double-precision%29) (InputAction :type Input%20Action%20Object%20Reference :default "/Game/Inputs/InputActions/IA_Rotation.IA_Rotation"))
  (Transformation|AddActorLocalRotation (Math|Rotator|MakeRotator (* ActionValue 5.0) 0.0 0.0) false false))

(event Input|EnhancedActionEvents|EnhancedInputActionIA_BrakeComboRight
  (params (ActionValue :type Boolean) (ElapsedSeconds :type Float%20%28double-precision%29) (TriggeredSeconds :type Float%20%28double-precision%29) (InputAction :type Input%20Action%20Object%20Reference :default "/Game/Inputs/InputActions/IA_BrakeComboRight.IA_BrakeComboRight")))

(event EventBeginPlay)

(event Collision|EventActorBeginOverlap
  (params (OtherActor :type Actor%20Object%20Reference)))

(event EventTick
  (params (DeltaSeconds :type Float%20%28single-precision%29)))

(fn ConstructionScript)