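; Player controller that owns the player's fixed-slot item inventory, pause input and movement input contexts.
; BeginPlay adds zero-G and debug Enhanced Input contexts, caches pawn and HUD, and clears the game-over flag; unlocking the jetpack swaps zero-G for jetpack controls.
; Slot cycling wraps around, updating the pawn's held item and HUD selection.
; Pickups fill the current slot, placing any previous occupant at the new item's transform.
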(event Custom|UnlockJetpack
  (bind _returnvalue (PlayerController|LocalPlayerSubsystems|GetEnhancedInputLocalPlayerSubsystem))
  ;[0.15 0.15 0.15 0.5] Unlock jetpack et affichage speedometre
  (Input|RemoveMappingContext _returnvalue "/Game/Inputs/IM_ZeroG.IM_ZeroG" "(bIgnoreAllPressedKeysUntilRelease=True,bForceImmediately=False,bNotifyUserSettings=False)")
  (Input|AddMappingContext _returnvalue "/Game/Inputs/IM_Jetpack.IM_Jetpack" 0 "(bIgnoreAllPressedKeysUntilRelease=True,bForceImmediately=False,bNotifyUserSettings=False)"))

(event Input|EnhancedActionEvents|EnhancedInputActionIA_ChangeCurrentItem
  (params (ActionValue :type Float%20%28double-precision%29) (ElapsedSeconds :type Float%20%28double-precision%29) (TriggeredSeconds :type Float%20%28double-precision%29) (InputAction :type Input%20Action%20Object%20Reference :default "/Game/Inputs/InputActions/IA_ChangeCurrentItem.IA_ChangeCurrentItem"))
  ;[0.15 0.15 0.15 0.5] Change current item
  (Variables|Default|SetCurrentItemIndex (+ ActionValue (Variables|Default|GetCurrentItemIndex)))
  (if (> (Math|Integer|%(Integer) (Variables|Default|GetCurrentItemIndex) (Variables|Default|GetInventoryMaxSlots)) -1)
    (bind _output_get (Variables|Default|SetCurrentItemIndex (Math|Integer|%(Integer) (Variables|Default|GetCurrentItemIndex) (Variables|Default|GetInventoryMaxSlots))))
    (else
      (Variables|Default|SetCurrentItemIndex (- (Variables|Default|GetInventoryMaxSlots) 1))))
  (Default|ChangeHeldItem (Variables|Default|GetPlayerActor) (Utilities|Array|Get(acopy) (Variables|Default|GetInventory) _output_get))
  (Default|ChangeSelectedItem (Variables|Default|GetAs%20HUD%20Game) _output_get))

(event Input|EnhancedActionEvents|EnhancedInputActionIA_PauseGame
  (params (ActionValue :type Boolean) (ElapsedSeconds :type Float%20%28double-precision%29) (TriggeredSeconds :type Float%20%28double-precision%29) (InputAction :type Input%20Action%20Object%20Reference :default "/Game/Inputs/InputActions/IA_PauseGame.IA_PauseGame"))
  ;[0.15 0.15 0.15 0.5] Appel du menu pause
  (:Started
    (Default|PauseGameMenu (Variables|Default|GetAs%20HUD%20Game))))

(event Input|EnhancedActionEvents|EnhancedInputActionIA_GiveJetpack
  (params (ActionValue :type Boolean) (ElapsedSeconds :type Float%20%28double-precision%29) (TriggeredSeconds :type Float%20%28double-precision%29) (InputAction :type Input%20Action%20Object%20Reference :default "/Game/Inputs/InputActions/Debug/IA_GiveJetpack.IA_GiveJetpack"))
  ;[0.15 0 0.1301 0.502] Comment
  (CallFunction|UnlockJetpack))

(event EventBeginPlay
  (bind _returnvalue (PlayerController|LocalPlayerSubsystems|GetEnhancedInputLocalPlayerSubsystem))
  (Utilities|IsValid _returnvalue
    (:Is%20Valid
      (Input|AddMappingContext _returnvalue "/Game/Inputs/IM_ZeroG.IM_ZeroG" 1 "(bIgnoreAllPressedKeysUntilRelease=True,bForceImmediately=False,bNotifyUserSettings=False)")
      (Input|AddMappingContext _returnvalue "/Game/Inputs/IM_Debug.IM_Debug" 2 "(bIgnoreAllPressedKeysUntilRelease=True,bForceImmediately=False,bNotifyUserSettings=False)")
      (bind _asbp_player (Utilities|Casting|CastToBP_Player (Game|Player|GetPlayerPawn 0)))
      (Variables|Default|SetPlayerActor _asbp_player)
      ;[0.15 0.15 0.15 0.5] Set HUD
      (bind _ashud_game (Utilities|Casting|CastToHUD_Game (HUD|GetHUD)))
      (Variables|Default|SetAs%20HUD%20Game _ashud_game)
      (Input|SetInputModeGameOnly self false)
      (bind _asgi_main (Utilities|Casting|CastToGI_Main (Game|GetGameInstance)))
      (Variables|/Game/BPs/GI_Main.GI_Main_C|SetIsGameOver _asgi_main false)
      (for _index (range 0 (- (Variables|Default|GetInventoryMaxSlots) 1))
        (Utilities|Array|Add (Variables|Default|GetInventory) 0)))))

(fn ConstructionScript)

(fn AddtoInventory
  (params (Item :type BP%20Item%20Pickable%20Object%20Reference))
  (bind _inventory (Variables|Default|GetInventory))
  (bind _currentitemindex (Variables|Default|GetCurrentItemIndex))
  (bind _output (Utilities|Array|Get(acopy) _inventory _currentitemindex))
  (bind _output_get (LocalVariables|SetLocalItemToAdd Item))
  (Default|ChangeHeldItem (Variables|Default|GetPlayerActor) _output_get)
  (Default|ChangeInventoryCellTexture (Variables|Default|GetAs%20HUD%20Game) (Variables|/Game/BPs/PickableObjects/BP_ItemPickable.BP_ItemPickable_C|GetInvetoryThumbnail _output_get) (Variables|Default|GetCurrentItemIndex))
  (if (not (Utilities|IsValid (Utilities|Array|Get(acopy) (Variables|Default|GetInventory) (Variables|Default|GetCurrentItemIndex))))
    (Utilities|Array|SetArrayElem (Variables|Default|GetInventory) (Variables|Default|GetCurrentItemIndex) (LocalVariables|GetLocalItemToAdd))
    (Collision|SetActorEnableCollision (LocalVariables|GetLocalItemToAdd) false)
    (Variables|/Game/BPs/PickableObjects/BP_ItemPickable.BP_ItemPickable_C|SetIsHeld (LocalVariables|GetLocalItemToAdd) true)
    (return true)
    (else
      (Rendering|SetActorHiddenInGame _output false)
      (Collision|SetActorEnableCollision _output true)
      (Transformation|SetActorTransform _output (Transformation|GetActorTransform (LocalVariables|GetLocalItemToAdd)))
      (Collision|SetActorEnableCollision (LocalVariables|GetLocalItemToAdd) false)
      (Variables|/Game/BPs/PickableObjects/BP_ItemPickable.BP_ItemPickable_C|SetIsHeld (LocalVariables|GetLocalItemToAdd) true)
      (Utilities|Array|SetArrayElem (Variables|Default|GetInventory) (Variables|Default|GetCurrentItemIndex) (LocalVariables|GetLocalItemToAdd))
      (return false))))

(fn DebugPrintAllInventroyItems
  (for _array_element (Variables|Default|GetInventory)
    (Development|PrintString (Utilities|GetDisplayName _array_element))))

(fn RemoveCurrentItemfromInventory
  (Utilities|Array|SetArrayElem (Variables|Default|GetInventory) (Variables|Default|GetCurrentItemIndex) 0)
  (Development|PrintString "RemoveItemFrommInventoryArray")
  (Default|ChangeInventoryCellTexture (Variables|Default|GetAs%20HUD%20Game) 0 (Variables|Default|GetCurrentItemIndex)))