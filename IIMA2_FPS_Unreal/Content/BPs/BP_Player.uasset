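; Player pawn with six-axis, momentum-based thruster movement, including roll and braking, that can grab surfaces, interact with objects and use or throw held items.
; Grabbing traces forward and timeline-lerps the pawn to the hit surface; releasing launches it along its facing direction.
; Hard box hits store a reflected velocity that Tick applies as a bounce, alongside held-item placement and hover traces.
; Throws preview the predicted path with spline meshes, then add a projectile component to the item.
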(event OnComponentHit(BoxPhysic)
  (params (HitComponent :type Primitive%20Component%20Object%20Reference) (OtherActor :type Actor%20Object%20Reference) (OtherComp :type Primitive%20Component%20Object%20Reference) (NormalImpulse :type Vector :default "0, 0, 0") (Hit :type Hit%20Result%20Structure%20%28by%20ref%29))
  (bind _returnvalue (Transformation|GetVelocity))
  (bind _returnvalue_2 (Math|Vector|Normalize _returnvalue))
  (bind _returnvalue_3 (Math|Vector|VectorLength _returnvalue))
  (bind _returnvalue_4 (Math|Vector|DotProduct (.normal Hit) _returnvalue_2))
  (bind _returnvalue_5 (* _returnvalue_4 -1.0))
  (bind _returnvalue_6 (* 1.0 _returnvalue_3 _returnvalue_5))
  ;[0.15 0.15 0.15 0.5] Impact
  (if (and (>= (* _returnvalue_5 9e+01) (Variables|Bounce|GetAngleToBounce)) (> _returnvalue_6 (Variables|Bounce|GetBounceImpactForceTreshold)))
    (Variables|Bounce|SetShouldBounce true)
    (Variables|Bounce|SetBounceVelocity (Math|Vector|GetReflectionVector (Variables|/Script/Engine.MovementComponent|GetVelocity (Variables|Default|GetFloatingPawnMovement)) (.normal Hit))))
  (if (> _returnvalue_6 (Variables|Miscellaneous|GetBonkThreshold))
    (Utilities|FlowControl|DoOnce false :!label _label
      (:Completed
        (Development|PrintString "WHOA")
        (Audio|SpawnSoundatLocation "/Game/Assets/Sounds/metal_pipe_falling_sound_effect.metal_pipe_falling_sound_effect" (Transformation|GetActorLocation) "0, 0, 0" 1.0 1.0 0.0 0 0)
        (Utilities|FlowControl|Delay 1.0)
        (goto _label Reset)))))

(event Input|EnhancedActionEvents|EnhancedInputActionIA_Braking
  (params (ActionValue :type Boolean) (ElapsedSeconds :type Float%20%28double-precision%29) (TriggeredSeconds :type Float%20%28double-precision%29) (InputAction :type Input%20Action%20Object%20Reference :default "/Game/Inputs/InputActions/IA_Braking.IA_Braking"))
  (bind _returnvalue (Transformation|GetVelocity))
  ;[0.15 0.15 0.15 0.5] Braking
  (if (< (Math|Vector|VectorLengthSquared _returnvalue) (Variables|Movement|GetBrakingSpeedThreshold))
    (Variables|/Script/Engine.MovementComponent|SetVelocity (Variables|Default|GetFloatingPawnMovement) "0, 0, 0")
    (else
      (Utilities|AddVelocity (* (* (Math|Vector|Normalize _returnvalue) (* (Variables|Movement|GetBrakingForce) (Utilities|Time|GetWorldDeltaSeconds))) -1.0)))))

(event Input|EnhancedActionEvents|EnhancedInputActionIA_Forward
  (params (ActionValue :type Float%20%28double-precision%29) (ElapsedSeconds :type Float%20%28double-precision%29) (TriggeredSeconds :type Float%20%28double-precision%29) (InputAction :type Input%20Action%20Object%20Reference :default "/Game/Inputs/InputActions/IA_Forward.IA_Forward"))
  ;[0.15 0.15 0.15 0.5] Déplacement
  (if (not (Variables|Grab|GetIsAttached))
    (Utilities|AddVelocity (* (* (Transformation|GetActorForwardVector) ActionValue) (* (Utilities|Time|GetWorldDeltaSeconds) (Variables|Movement|GetThrusterSpeed))))))

(event Input|EnhancedActionEvents|EnhancedInputActionIA_Throw
  (params (ActionValue :type Boolean) (ElapsedSeconds :type Float%20%28double-precision%29) (TriggeredSeconds :type Float%20%28double-precision%29) (InputAction :type Input%20Action%20Object%20Reference :default "/Game/Inputs/InputActions/IA_Throw.IA_Throw"))
  (:Triggered
    ;[0.15 0.15 0.15 0.5] prévisualisation
    (Development|PrintString "Hello")
    (CallFunction|RemoveSplineMeshes)
    (bind _outpathpositions (Class|GameplayStatics|BlueprintPredictProjectilePathbyTraceChannel (Transformation|GetWorldLocation (Variables|Default|GetHeldObjectPlacement)) (* (Transformation|GetActorForwardVector) (Variables|Items|GetThrowForce)) true 1e+01 "ECC_GameTraceChannel4" false 0 "ForOneFrame" 0.0 1e+01 3.0))
    (Spline|SetSplinePoints (Variables|Default|GetThrowPrevisualisation) _outpathpositions "World" true)
    (CallFunction|AddSplineMeshes))
  (:Completed
    ;[0.15 0.15 0.15 0.5] Throw
    (Development|PrintString "throw")
    (Utilities|IsValid (Variables|Items|GetHoldedItem)
      (:Is%20Valid
        (bind _returnvalue (AddComponent|AddProjectileMovementComponent (Variables|Items|GetHoldedItem)))
        (Utilities|SetProjectileComponent _returnvalue
          (:OutExec
            (Variables|/Game/BPs/PickableObjects/BP_ItemPickable.BP_ItemPickable_C|SetProjectileComponent (Variables|Items|GetHoldedItem) _returnvalue)
            (Components|Activation|Activate _returnvalue false)
            (Variables|/Script/Engine.MovementComponent|SetVelocity _returnvalue (* (Transformation|GetActorForwardVector) (Variables|Items|GetThrowForce)))
            (Collision|SetActorEnableCollision (Variables|Items|GetHoldedItem) true)
            (Variables|Items|SetHoldedItem 0)
            (Default|RemoveCurrentItemfromInventory (Variables|Miscellaneous|GetPlayerController)))))
      (:Is%20Not%20Valid
        _))
    (CallFunction|RemoveSplineMeshes)))

(event Input|EnhancedActionEvents|EnhancedInputActionIA_Grab
  (params (ActionValue :type Boolean) (ElapsedSeconds :type Float%20%28double-precision%29) (TriggeredSeconds :type Float%20%28double-precision%29) (InputAction :type Input%20Action%20Object%20Reference :default "/Game/Inputs/InputActions/IA_Grab.IA_Grab"))
  (bind _returnvalue (Transformation|GetActorLocation))
  ;[0.15 0.15 0.15 0.5] Grab
  (:Started
    (bind (_outhit _returnvalue_2) (Collision|LineTraceByChannel _returnvalue (+ _returnvalue (* (Transformation|GetActorForwardVector) (Variables|Grab|GetGrabRange))) "TraceTypeQuery3" false 0 "ForOneFrame"))
    (if _returnvalue_2
      (Variables|/Script/Engine.MovementComponent|SetVelocity (Variables|Default|GetFloatingPawnMovement) "0, 0, 0")
      (Variables|Grab|SetIsAttached true)
      (Variables|Miscellaneous|SetTempPlayerPos (Transformation|GetActorLocation))
      (bind _time (Timeline|GrabAnimation PlayFromStart)
        (:Update
          (if (Variables|Grab|GetIsAttached)
            (Transformation|SetActorLocation (Math|Vector|Lerp(Vector) (Variables|Miscellaneous|GetTempPlayerPos) (+ (.impactpoint _outhit) (* (.impactnormal _outhit) (Variables|Grab|GetDistanceFromGrabable))) _time) false false)
            (else
              (Audio|Components|Audio|Stop (Variables|Default|GetGrabAnimation))))))))
  (:Completed
    (if (Variables|Grab|GetIsAttached)
      (Utilities|AddVelocity (* (Transformation|GetActorForwardVector) (Variables|Movement|GetJumpSpeed))
        (:Exec
          (Variables|Grab|SetIsAttached false))))))

(event Input|EnhancedActionEvents|EnhancedInputActionIA_Strafe
  (params (ActionValue :type Float%20%28double-precision%29) (ElapsedSeconds :type Float%20%28double-precision%29) (TriggeredSeconds :type Float%20%28double-precision%29) (InputAction :type Input%20Action%20Object%20Reference :default "/Game/Inputs/InputActions/IA_Strafe.IA_Strafe"))
  ;[0.15 0.15 0.15 0.5] Déplacement latéral
  (if (not (Variables|Grab|GetIsAttached))
    (Utilities|AddVelocity (* (* (Transformation|GetActorRightVector) ActionValue) (* (Utilities|Time|GetWorldDeltaSeconds) (Variables|Movement|GetThrusterSpeed))))))

(event Input|EnhancedActionEvents|EnhancedInputActionIA_Elevation
  (params (ActionValue :type Float%20%28double-precision%29) (ElapsedSeconds :type Float%20%28double-precision%29) (TriggeredSeconds :type Float%20%28double-precision%29) (InputAction :type Input%20Action%20Object%20Reference :default "/Game/Inputs/InputActions/IA_Elevation.IA_Elevation"))
  ;[0.15 0.15 0.15 0.5] Elevation
  (if (not (Variables|Grab|GetIsAttached))
    (Utilities|AddVelocity (* (* (Transformation|GetActorUpVector) ActionValue) (* (Utilities|Time|GetWorldDeltaSeconds) (Variables|Movement|GetThrusterSpeed))))))

(event Input|EnhancedActionEvents|EnhancedInputActionIA_Look
  (params (ActionValue :type Vector%202D%20Structure) (ElapsedSeconds :type Float%20%28double-precision%29) (TriggeredSeconds :type Float%20%28double-precision%29) (InputAction :type Input%20Action%20Object%20Reference :default "/Game/Inputs/InputActions/IA_Look.IA_Look"))
  (bind _returnvalue (Utilities|Time|GetWorldDeltaSeconds))
  (bind _camerasensibility (Variables|Movement|GetCameraSensibility))
  (bind _returnvalue_2 (* _camerasensibility _returnvalue))
  ;[0.15 0.15 0.15 0.5] Camera
  (Transformation|AddActorLocalRotation (Math|Rotator|MakeRotator 0.0 (* (.y ActionValue) _returnvalue_2) (* (.x ActionValue) _returnvalue_2)) false false))

(event Input|EnhancedActionEvents|EnhancedInputActionIA_Rotation
  (params (ActionValue :type Float%20%28double-precision%29) (ElapsedSeconds :type Float%20%28double-precision%29) (TriggeredSeconds :type Float%20%28double-precision%29) (InputAction :type Input%20Action%20Object%20Reference :default "/Game/Inputs/InputActions/IA_Rotation.IA_Rotation"))
  ;[0.15 0.15 0.15 0.5] Rotation
  (Transformation|AddActorLocalRotation (Math|Rotator|MakeRotator (* ActionValue (* (Variables|Movement|GetRotationSpeed) (Utilities|Time|GetWorldDeltaSeconds))) 0.0 0.0) false false))

(event Input|EnhancedActionEvents|EnhancedInputActionIA_UseItem
  (params (ActionValue :type Boolean) (ElapsedSeconds :type Float%20%28double-precision%29) (TriggeredSeconds :type Float%20%28double-precision%29) (InputAction :type Input%20Action%20Object%20Reference :default "/Game/Inputs/InputActions/IA_UseItem.IA_UseItem"))
  (bind _holdeditem (Variables|Items|GetHoldedItem))
  ;[0.15 0.15 0.15 0.5] UseItem
  (:Started
    (Utilities|IsValid _holdeditem
      (:Is%20Valid
        (Default|UseItem _holdeditem)))))

(event Input|EnhancedActionEvents|EnhancedInputActionIA_Debug
  (params (ActionValue :type Boolean) (ElapsedSeconds :type Float%20%28double-precision%29) (TriggeredSeconds :type Float%20%28double-precision%29) (InputAction :type Input%20Action%20Object%20Reference :default "/Game/Inputs/InputActions/IA_Debug.IA_Debug"))
  ;[0.15 0 0.1308 0.5] Debug
  (Development|PrintString (Utilities|String|ToString(Float) (Math|Vector|VectorLength (Transformation|GetVelocity)))))

(event Input|EnhancedActionEvents|EnhancedInputActionIA_Interact
  (params (ActionValue :type Boolean) (ElapsedSeconds :type Float%20%28double-precision%29) (TriggeredSeconds :type Float%20%28double-precision%29) (InputAction :type Input%20Action%20Object%20Reference :default "/Game/Inputs/InputActions/IA_Interact.IA_Interact"))
  (bind _returnvalue (Transformation|GetActorLocation))
  (:Completed
    (bind _outhit (Collision|LineTraceByChannel _returnvalue (+ _returnvalue (* (Transformation|GetActorForwardVector) (Variables|Grab|GetGrabRange))) "TraceTypeQuery4" false 0 "None"))
    (Class|BPIInteractable|OnInteracte(Message) (.hitactor _outhit))))

(event EventBeginPlay
  (Components|Timeline|SetPlayRate (Variables|Default|GetGrabAnimation) (Variables|Grab|GetGrabSpeedAnimation))
  (bind _aspc_player (Utilities|Casting|CastToPC_Player (Game|GetPlayerController 0)))
  (Variables|Miscellaneous|SetPlayerController _aspc_player))

(event EventTick
  (params (DeltaSeconds :type Float%20%28single-precision%29))
  (bind _returnvalue (Transformation|GetActorLocation))
  (bind _returnvalue_2 (Transformation|GetActorLocation))
  ;[0.15 0.15 0.15 0.5] Réticule visuel et interactibles OnHover
  (Utilities|HoldIteminHand
    (:OutExec
      (Utilities|ShouldBounceThisTick
        (:OutputExec
          ;;[0.15 0.15 0.15 0.5] Visuel du réticule de grab et objets
          (Collision|LineTraceByChannel _returnvalue_2 (+ _returnvalue_2 (* (Transformation|GetActorForwardVector) (Variables|Grab|GetGrabRange))) "TraceTypeQuery3" false 0 "ForOneFrame")
          (bind (_outhit _returnvalue_3) (Collision|LineTraceByChannel _returnvalue (+ _returnvalue (* (Transformation|GetActorForwardVector) (Variables|Grab|GetGrabRange))) "TraceTypeQuery4" false 0 "ForOneFrame" true "(R=1.000000,G=0.000000,B=0.829622,A=1.000000)" "(R=0.317070,G=0.000000,B=1.000000,A=1.000000)"))
          (if _returnvalue_3
            (Class|BPIInteractable|OnHover(Message) (.hitactor _outhit))))))))

(fn ConstructionScript)

(fn ChangeHeldItem
  (params (NewHeldItem :type BP%20Item%20Pickable%20Object%20Reference))
  (Utilities|IsValid NewHeldItem
    (:Is%20Valid
      (Utilities|IsValid (Variables|Items|GetHoldedItem)
        (:Is%20Valid
          (Rendering|SetActorHiddenInGame (Variables|Items|GetHoldedItem) true))
        (:Is%20Not%20Valid
          _))
      (bind _output_get (Variables|Items|SetHoldedItem NewHeldItem))
      (Rendering|SetActorHiddenInGame _output_get false)
      (return))
    (:Is%20Not%20Valid
      (Utilities|IsValid (Variables|Items|GetHoldedItem)
        (:Is%20Valid
          (Rendering|SetActorHiddenInGame (Variables|Items|GetHoldedItem) true)
          (return))))))

(fn RemoveBounce
  (Variables|Bounce|SetBounceImpactForceTreshold 999999999.0))

(fn AddSplineMeshes
  (bind _throwprevisualisation (Variables|Default|GetThrowPrevisualisation))
  (bind _throwprevisualisation_2 (Variables|Default|GetThrowPrevisualisation))
  (Transformation|SetMobility (Variables|Default|GetBoxPhysic) "Static")
  (for _index (range 0 (- (Spline|GetNumberOfSplinePoints (Variables|Default|GetThrowPrevisualisation)) 2))
    (if (> (- (Spline|GetDistanceAlongSplineatSplinePoint _throwprevisualisation (+ _index 1)) (Spline|GetDistanceAlongSplineatSplinePoint _throwprevisualisation _index)) (Variables|Items|GetThrowMinDistance))
      (bind _returnvalue (AddComponent|AddSplineMeshComponent false))
      (bind _output_get (LocalVariables|SetSSMC _returnvalue))
      (Transformation|SetMobility _output_get "Movable")
      (Collision|SetCollisionEnabled _output_get "NoCollision")
      (Collision|SetCollisionResponsetoAllChannels _output_get "ECR_Ignore")
      (Utilities|Array|Add (Variables|Items|GetSplineMeshesList) _output_get)
      (Components|StaticMesh|SetStaticMesh _output_get (Variables|Items|GetPrevisualisationMesh))
      (SplineMesh|SetStartandEnd (LocalVariables|GetSSMC) (.Location (Spline|GetLocationandTangentatSplinePoint _throwprevisualisation_2 _index "Local")) (.Tangent (Spline|GetLocationandTangentatSplinePoint _throwprevisualisation_2 _index "Local")) (.Location (Spline|GetLocationandTangentatSplinePoint _throwprevisualisation_2 (+ _index 1) "Local")) (.Tangent (Spline|GetLocationandTangentatSplinePoint _throwprevisualisation_2 (+ _index 1) "Local")) true :!class /Script/Engine.SplineMeshComponent)
      (SplineMesh|SetForwardAxis (LocalVariables|GetSSMC) "Z" false)
      (SplineMesh|SetStartScale (LocalVariables|GetSSMC) "(X=1.000000,Y=1.000000)" false :!class /Script/Engine.SplineMeshComponent)
      (SplineMesh|SetEndScale (LocalVariables|GetSSMC) "(X=1.000000,Y=1.000000)" false :!class /Script/Engine.SplineMeshComponent)))
  (Transformation|SetMobility (Variables|Default|GetBoxPhysic) "Movable"))

(fn RemoveSplineMeshes
  (for _array_element (Variables|Items|GetSplineMeshesList)
    (Components|DestroyComponent _array_element))
  (Utilities|Array|Clear (Variables|Items|GetSplineMeshesList)))